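; Paper2D platform that burns away when the player touches it with a high enough flame, losing collision and hiding after a delay.
; A self-calling event then burns the linked platforms one after another, and the chain ends by lighting a connected brazier or small torch.
; The burn effect swaps the sprite material and timestamps a shared Material Parameter Collection.
; An older DelayedLoop version of the chain remains unwired, marked for removal.
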(event `self.ReceiveBeginPlay`
  (`|ExecutionSequence`
    (:`then_0`
      (if (!= (`KismetArrayLibrary.Array_Length` (`self.ConnectedPlatforms`)) 0)
        (set `self.IsConnectedToOther` true)
        (else
          (`KismetArrayLibrary.Array_Clear` (`self.ConnectedPlatforms`))
          (set `self.IsConnectedToOther` false))))
    (:`then_1`
      (`/Engine/EditorBlueprintResources/StandardMacros.IsValid` (`self.ConnectedTorch`)
        (:`Is Valid`
          (set `self.IsTorchConnected` true))
        (:`Is Not Valid`
          (`/Engine/EditorBlueprintResources/StandardMacros.IsValid` (`self.ConnectedSmallTorch`)
            (:`Is Valid`
              (set `self.IsSmallTorchConnected` true))
            (:`Is Not Valid`
              (set `self.IsTorchConnected` false)
              (set `self.IsSmallTorchConnected` false))))))
    (:`then_2`
      (set `self.BaseMaterial` (`PrimitiveComponent.GetMaterial` (`self.PaperSprite`) 0)))))

(event `self.Trigger.OnComponentBeginOverlap`
  (params (OverlappedComponent :type "PrimitiveComponent Object Reference") (OtherActor :type "Actor Object Reference") (OtherComp :type "PrimitiveComponent Object Reference") (OtherBodyIndex :type Integer) (bFromSweep :type Boolean) (SweepResult :type "HitResult Structure (by ref)"))
  (bind _asbp_player (cast `/Game/Characters/Player/Blueprints/BP_Player` OtherActor))
  (set `self.BPPlayer` _asbp_player)
  (bind _returnvalue (`self.HasHighFlame`))
  (if (and _returnvalue (not (`self.IsBurning`)))
    (`PrimitiveComponent.SetCollisionResponseToAllChannels` (`self.Collision`) "ECR_Ignore")
    (`PrimitiveComponent.SetCollisionResponseToAllChannels` (`self.Trigger`) "ECR_Ignore")
    (set `self.IsBurning` true)
    (`self.ActivateBurningMaterial`)
    (if (`self.IsConnectedToOther`)
      (if (< (`self.IndexElement`) (`KismetArrayLibrary.Array_Length` (`self.ConnectedPlatforms`)))
        (`self.NextArrayElement` (`|GetArrayItem` (`self.ConnectedPlatforms`) (`self.IndexElement`)))
        (else
          (if (`self.IsTorchConnected`) :!label _label
            (`/Game/Prototype/Blueprints/BP_FlameForDoor.LightBrasero` (`self.ConnectedTorch`))
            (elif (`self.IsSmallTorchConnected`)
              (`/Game/Prototype/Blueprints/BP_FlameForSmallDoorV2.TorchLitByFlamable` (`self.ConnectedSmallTorch`))))))
      (else
        (goto _label)))))

(event `NextArrayElement`
  (params (ConnectedFlamableElement :type "/Game/Prototype/Blueprints/BP_FlamablePlatform Object Reference"))
  (bind _papersprite (`/Game/Prototype/Blueprints/BP_FlamablePlatform.PaperSprite` ConnectedFlamableElement))
  (set `/Game/Prototype/Blueprints/BP_FlamablePlatform.IsBurning` true ConnectedFlamableElement)
  (`GameplayStatics.PlaySound2D` "/Game/Sounds/PlatformFlamable_Cue.PlatformFlamable_Cue" 1.0 1.0 0.0 null null)
  (`PrimitiveComponent.SetCollisionResponseToAllChannels` (`/Game/Prototype/Blueprints/BP_FlamablePlatform.Collision` ConnectedFlamableElement) "ECR_Ignore")
  (`PrimitiveComponent.SetCollisionResponseToAllChannels` (`/Game/Prototype/Blueprints/BP_FlamablePlatform.Trigger` ConnectedFlamableElement) "ECR_Ignore")
  ;[0.4412 0.4412 0.4412] Active burning material
  (`PrimitiveComponent.SetMaterial` _papersprite 0 (`self.BurnMat`))
  (`KismetMaterialLibrary.SetScalarParameterValue` "/Game/Materials/FlamablePlatform/MPC_BurningMaterial.MPC_BurningMaterial" "HitTime" (`KismetSystemLibrary.GetGameTimeInSeconds`))
  (`KismetSystemLibrary.Delay` (`self.DelayBeforeDisapearing`))
  (`PrimitiveComponent.SetMaterial` _papersprite 0 (`self.BaseMaterial`))
  (`SceneComponent.SetVisibility` _papersprite false false)
  (set `self.IndexElement` (+ (`self.IndexElement`) 1))
  (if (< (`self.IndexElement`) (`KismetArrayLibrary.Array_Length` (`self.ConnectedPlatforms`)))
    (`self.NextArrayElement` (`|GetArrayItem` (`self.ConnectedPlatforms`) (`self.IndexElement`)))
    (else
      (goto _label))))

(fn `HasHighFlame`
  (returns (ReturnValue :type Boolean))
  (return (>= (`FlameComponent.GetFlameValue` (`/Game/Characters/Player/Blueprints/BP_Player.Flame` (`self.BPPlayer`))) 70.0)))

(fn `UserConstructionScript`)