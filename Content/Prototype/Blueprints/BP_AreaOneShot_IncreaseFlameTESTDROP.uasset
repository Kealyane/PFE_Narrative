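; BP_AreaOneShot_IncreaseFlameTESTDROP is a prototype area trigger that temporarily disables itself after a PFECharacter overlaps it.
; One second after the overlap, its Cube switches to a disabled material and ignores the Pawn channel, then reverts after DisableDuration.
; BeginPlay passes Sound to InitSoundComponent; the graph itself contains no flame-increase logic, despite the name.
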(event `self.ReceiveBeginPlay`
  (`self.InitSoundComponent` (`self.Sound`)))

(event `self.ReceiveActorBeginOverlap`
  (params (OtherActor :type "Actor Object Reference"))
  (cast `PFECharacter` OtherActor)
  (`KismetSystemLibrary.Delay` 1.0)
  (`PrimitiveComponent.SetMaterial` (`self.Cube`) 0 "/Game/Materials/M_DisabledPoint.M_DisabledPoint")
  (`PrimitiveComponent.SetCollisionResponseToChannel` (`self.Cube`) "ECC_Pawn" "ECR_Ignore")
  (`KismetSystemLibrary.Delay` (`self.DisableDuration`))
  (`PrimitiveComponent.SetMaterial` (`self.Cube`) 0 "/Game/Materials/M_Point-.M_Point-")
  (`PrimitiveComponent.SetCollisionResponseToChannel` (`self.Cube`) "ECC_Pawn" "ECR_Overlap"))

(fn `UserConstructionScript`)