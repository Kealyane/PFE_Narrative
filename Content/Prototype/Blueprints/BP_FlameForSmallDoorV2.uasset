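; Brazier prototype for a small-door puzzle: overlapping player's flame value decides its reaction and updates the linked door's active-flame count.
; A low flame lights it once until reset; a middle one puts out a lit brazier or flashes wrong-flame feedback.
; A high flame triggers an explosion that briefly hides the brazier and disables its collision.
; TorchLitByFlamable runs the extinguish path directly, despite its name.
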(event `self.ReceiveActorBeginOverlap`
  (params (OtherActor :type "Actor Object Reference"))
  (bind _affiliateddoor (`self.AffiliatedDoor`))
  (bind _affiliateddoor_2 (`self.AffiliatedDoor`))
  (bind _wrongflamefeedback (`self.WrongFlameFeedback`))
  (bind _asbp_player (cast `/Game/Characters/Player/Blueprints/BP_Player` OtherActor))
  (set `self.PlayerRef` _asbp_player)
  (if (>= (`FlameComponent.GetFlameValue` (`/Game/Characters/Player/Blueprints/BP_Player.Flame` _asbp_player)) 70.0)
    (`self.Burnt`)
    (elif (<= (`FlameComponent.GetFlameValue` (`/Game/Characters/Player/Blueprints/BP_Player.Flame` _asbp_player)) 30.0)
      (`/Engine/EditorBlueprintResources/StandardMacros.DoOnce` false :!label _label
        (:`Completed`
          (`SceneComponent.SetVisibility` (`self.Flame`) true false)
          (`/Engine/EditorBlueprintResources/StandardMacros.IncrementInt` (`/Game/Prototype/Blueprints/BP_SmallFlameDoorV2.ActivatedFlames` _affiliateddoor)
            (:`  `
              (set `self.Out` true)
              (`GameplayStatics.PlaySoundAtLocation` "/Game/Interactables/Braseros/Sounds/BraseroLit.BraseroLit" (`SceneComponent.K2_GetComponentLocation` (`self.DefaultSceneRoot`)) (struct) 1.0 1.0 0.0 null null null null)
              (`/Game/Prototype/Blueprints/BP_SmallFlameDoorV2.CheckFlames` _affiliateddoor)))))
      (elif (`self.Out`)
        (`SceneComponent.SetVisibility` (`self.Flame`) false false :!label _label_2)
        (set `self.Out` false)
        (`GameplayStatics.PlaySoundAtLocation` "/Game/Interactables/Braseros/Sounds/BraseroOut.BraseroOut" (`SceneComponent.K2_GetComponentLocation` (`self.DefaultSceneRoot`)) (struct) 1.0 1.0 0.0 null null null null)
        (`/Engine/EditorBlueprintResources/StandardMacros.DecrementInt` (`/Game/Prototype/Blueprints/BP_SmallFlameDoorV2.ActivatedFlames` _affiliateddoor_2)
          (:`  `
            (`/Game/Prototype/Blueprints/BP_SmallFlameDoorV2.CheckFlames` _affiliateddoor_2)
            (`self.Reset`)))
        (else
          (`GameplayStatics.PlaySoundAtLocation` null (`SceneComponent.K2_GetComponentLocation` (`self.DefaultSceneRoot`)) (struct) 1.0 1.0 0.0 null null null null)
          (`SceneComponent.SetVisibility` _wrongflamefeedback true false)
          (`KismetSystemLibrary.Delay` 0.5)
          (`SceneComponent.SetVisibility` _wrongflamefeedback false false))))))

(event `Reset`
  (goto _label :!via `Reset`))

(event `TorchLitByFlamable`
  (goto _label_2))

(event `Burnt`
  (bind (_returnvalue_x _returnvalue_y _returnvalue_z) (`KismetMathLibrary.BreakVector` (`SceneComponent.K2_GetComponentLocation` (`self.DefaultSceneRoot`))))
  (bind _returnvalue (`|SpawnActorFromClass` "/Game/Blueprints/Misc/PlayerExplosion.PlayerExplosion_C" (`KismetMathLibrary.MakeTransform` (`KismetMathLibrary.MakeVector` _returnvalue_x 1011.0 _returnvalue_z) (struct) (3.0 3.0 3.0)) "Undefined" "MultiplyWithRoot" null null))
  (`/Game/Blueprints/Misc/PlayerExplosion.Called` _returnvalue)
  (`GameplayStatics.PlaySoundAtLocation` "/Game/Interactables/Braseros/Sounds/BraseroExploded.BraseroExploded" (`SceneComponent.K2_GetComponentLocation` (`self.DefaultSceneRoot`)) (struct) 1.0 1.0 0.0 null null null null)
  (`KismetSystemLibrary.Delay` 0.2)
  (`SceneComponent.SetVisibility` (`self.Pedestal`) false false)
  (`SceneComponent.SetVisibility` (`self.Flame`) false false)
  (`PrimitiveComponent.SetCollisionEnabled` (`self.Box`) "NoCollision")
  (`KismetSystemLibrary.Delay` 2.0)
  (`SceneComponent.SetVisibility` (`self.Pedestal`) true false)
  (`PrimitiveComponent.SetCollisionEnabled` (`self.Box`) "QueryOnly")
  (if (`self.Out`)
    (`SceneComponent.SetVisibility` (`self.Flame`) true false)))

(fn `UserConstructionScript`)