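; Trigger actor that plays an environment level sequence once when its box is overlapped, then resets it when the game mode broadcasts a death.
; On BeginPlay it binds Respawn to the PFEGameMode death event and caches the starting transforms of the SpritesUsed actors.
; Respawn waits briefly, stops the sequence player, restores those transforms and re-arms the trigger.
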(event `self.ReceiveBeginPlay`
  (bind _aspfegame_mode (cast `PFEGameMode` (`GameplayStatics.GetGameMode`)))
  (add `PFEGameMode.OnDeath` _aspfegame_mode (delegate `Respawn`))
  (for _array_element (`self.SpritesUsed`)
    (`KismetArrayLibrary.Array_Add` (`self.SpriteTransforms`) (`self.GetTransform` _array_element))))

(event `Respawn`
  (bind _sequence_player (`self.Sequence Player`))
  (`/Engine/EditorBlueprintResources/StandardMacros.IsValid` _sequence_player
    (:`Is Valid`
      (`KismetSystemLibrary.Delay` 1.0)
      (`MovieSceneSequencePlayer.Stop` _sequence_player)
      (set `self.HasPlayedSequence` false)
      (for (_array_element _array_index) (`self.SpritesUsed`)
        (`self.K2_SetActorTransform` _array_element (`|GetArrayItem` (`self.SpriteTransforms`) _array_index) false false)))))

(event `self.Box.OnComponentBeginOverlap`
  (params (OverlappedComponent :type "PrimitiveComponent Object Reference") (OtherActor :type "Actor Object Reference") (OtherComp :type "PrimitiveComponent Object Reference") (OtherBodyIndex :type Integer) (bFromSweep :type Boolean) (SweepResult :type "HitResult Structure (by ref)"))
  (if (not (`self.HasPlayedSequence`))
    (bind _outactor (`LevelSequencePlayer.CreateLevelSequencePlayer` (`self.SequenceToPlay`)))
    (bind _output_get (set `self.Sequence Player` (`LevelSequenceActor.SequencePlayer` _outactor)))
    (`MovieSceneSequencePlayer.Play` _output_get)
    (set `self.HasPlayedSequence` true)))

(fn `UserConstructionScript`)