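; Trigger actor that plays an assigned level sequence, likely a pillar set piece, when the player enters its box.
; BeginPlay creates the sequence player and binds Reset to the game mode's death event.
; A DoOnce gates the overlap ahead of the player cast, and the box's collision turns off once triggered.
; On death, playback stops, then after short delays rewinds, restores collision and re-arms the DoOnce.
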(event `self.ReceiveBeginPlay`
  (bind (_outactor _returnvalue) (`LevelSequencePlayer.CreateLevelSequencePlayer` (`self.SequenceToPlay`)))
  (set `self.SequencePlayer` _returnvalue)
  (bind _aspfegame_mode (cast `PFEGameMode` (`GameplayStatics.GetGameMode`)))
  (add `PFEGameMode.OnDeath` _aspfegame_mode (delegate `Reset`)))

(event `self.Box.OnComponentBeginOverlap`
  (params (OverlappedComponent :type "PrimitiveComponent Object Reference") (OtherActor :type "Actor Object Reference") (OtherComp :type "PrimitiveComponent Object Reference") (OtherBodyIndex :type Integer) (bFromSweep :type Boolean) (SweepResult :type "HitResult Structure (by ref)"))
  (`/Engine/EditorBlueprintResources/StandardMacros.DoOnce` false :!label _label
    (:`Completed`
      (cast `/Game/Blueprints/Player/BP_Player` OtherActor)
      (`MovieSceneSequencePlayer.Play` (`LevelSequenceActor.SequencePlayer` (stale `self.ReceiveBeginPlay` _outactor)))
      (`PrimitiveComponent.SetCollisionEnabled` (`self.Box`) "NoCollision"))))

(event `Reboot`
  (goto _label :!via `Reset`))

(event `Reset`
  (`MovieSceneSequencePlayer.Stop` (`LevelSequenceActor.SequencePlayer` (stale `self.ReceiveBeginPlay` _outactor)))
  (`KismetSystemLibrary.Delay` 1.2)
  (`MovieSceneSequencePlayer.SetPlaybackPosition` (`LevelSequenceActor.SequencePlayer` (stale `self.ReceiveBeginPlay` _outactor)) (make `MovieSceneSequencePlaybackParams` (struct :`FrameNumber` (struct))))
  (`PrimitiveComponent.SetCollisionEnabled` (`self.Box`) "QueryOnly")
  (`KismetSystemLibrary.Delay` 0.5)
  (`self.Reboot`))

(fn `UserConstructionScript`)