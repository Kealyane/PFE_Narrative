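; BP_Checkpoint is a level checkpoint that records the player's progress and signals it with sound and a UI animation.
; On BeginPlay, after a short delay, it caches the interface widget, the game instance and the current level as an enum.
; When activated, it saves the checkpoint through the game instance if not already reached, then plays the sound and widget animation regardless.
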(event `self.ReceiveBeginPlay`
  (`KismetSystemLibrary.Delay` 0.5)
  (bind _foundwidgets (`WidgetBlueprintLibrary.GetAllWidgetsOfClass` "/Game/UI/Widgets/HUD/WBP_Interface.WBP_Interface_C" false))
  (set `self.Widget` (`|GetArrayItem` _foundwidgets))
  (bind _asbp_pfegame_instance (cast `/Game/Blueprints/Core/BP_PFEGameInstance` (`GameplayStatics.GetGameInstance`)))
  (set `self.MyGameInstance` _asbp_pfegame_instance)
  (bind _returnvalue (`GameplayStatics.GetCurrentLevelName` true))
  (bind _level (`/Game/Blueprints/Core/BP_PFEGameInstance.GetEnumFromPath` (`self.MyGameInstance`) _returnvalue))
  (set `self.CurrentLevel` _level))

(event `self.UpdateCheckpoint`
  (params (InIsActive :type Boolean))
  (if InIsActive
    (`self.SaveReachCheckpoint`)
    (`SoundComponent.PlaySound` (`self.Sound`) "Checkpoint")
    (`/Game/UI/Widgets/HUD/WBP_Interface.CallCheckpointAnim` (`self.Widget`))))

(fn `SaveReachCheckpoint`
  (bind _returnvalue (`PFEGameInstance.CheckHasReachCheckpoint` (`self.MyGameInstance`) (`self.CurrentLevel`)))
  (if (not _returnvalue)
    (`PFEGameInstance.SaveLevelCheckpoint` (`self.MyGameInstance`) (`self.CurrentLevel`) false))
  (return))

(fn `UserConstructionScript`)