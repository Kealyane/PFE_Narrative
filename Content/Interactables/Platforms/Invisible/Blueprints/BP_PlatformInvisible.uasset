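; BP_PlatformInvisible is an invisible platform paired with a mirror-image sprite, which selects its look, and vertical offset when IsVertical, at BeginPlay.
; Two update functions place the mirror sprite by reflecting the actor's position across an Axis actor horizontally or vertically, scaled by a distance multiplier.
; Player overlap spawns a Niagara mirror effect at the walkable platform, repeated by a looping timer until an overlap ends.
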(event `self.ReceiveBeginPlay`
  (bind _mirorplatform (`self.MirorPlatform`))
  (bind (_relativelocation_x _relativelocation_y) (`KismetMathLibrary.BreakVector` (`SceneComponent.RelativeLocation` _mirorplatform)))
  (if (`self.IsVertical`)
    (`PaperSpriteComponent.SetSprite` (`self.MirorPlatform`) (`self.SpriteNormal`))
    (`SceneComponent.K2_SetRelativeLocation` _mirorplatform (`KismetMathLibrary.MakeVector` _relativelocation_x _relativelocation_y -72.0) false false)
    (else
      (`PaperSpriteComponent.SetSprite` (`self.MirorPlatform`) (`self.SpriteInvert`)))))

(event `self.ReceiveActorBeginOverlap`
  (params (OtherActor :type "Actor Object Reference"))
  (bind (_returnvalue_x _returnvalue_y _returnvalue_z) (`KismetMathLibrary.BreakVector` (`SceneComponent.K2_GetComponentLocation` (`self.WalkablePlatform`))))
  (cast `/Game/Characters/Player/Blueprints/BP_Player` OtherActor)
  (set `self.StillOnPlatform` true)
  (bind _output_get (set `self.PlatformLoc` (`KismetMathLibrary.MakeVector` _returnvalue_x _returnvalue_y _returnvalue_z)))
  (`NiagaraFunctionLibrary.SpawnSystemAtLocation` "/Game/VFX/NS_MirrorPlatform.NS_MirrorPlatform" (`KismetMathLibrary.MakeVector` (.x _output_get) (.y _output_get) (.z _output_get)))
  (bind _returnvalue (`KismetSystemLibrary.K2_SetTimerDelegate` (delegate `CheckPlayerStillOnPlat`) 2.0 true))
  (set `self.Timer` _returnvalue))

(event `CheckPlayerStillOnPlat`
  (if (`self.StillOnPlatform`)
    (`NiagaraFunctionLibrary.SpawnSystemAtLocation` "/Game/VFX/NS_MirrorPlatform.NS_MirrorPlatform" (`self.PlatformLoc`))))

(event `self.ReceiveActorEndOverlap`
  (params (OtherActor :type "Actor Object Reference"))
  (set `self.StillOnPlatform` false)
  (`KismetSystemLibrary.K2_ClearAndInvalidateTimerHandle` (`self.Timer`)))

(fn `UpdateHorizontalMirrorPosition`
  (params (Axis :type "Actor Object Reference") (DistanceMultiplier :type "Float (double-precision)"))
  (locals (DistanceFromAxis :type "Float (double-precision)" :default 0.0))
  (bind (_returnvalue_x _returnvalue_y _returnvalue_z) (`KismetMathLibrary.BreakVector` (`self.K2_GetActorLocation` Axis)))
  (bind (_returnvalue_x_2 _returnvalue_y_2 _returnvalue_z_2) (`KismetMathLibrary.BreakVector` (`self.K2_GetActorLocation`)))
  (bind (_returnvalue_x_3 _returnvalue_y_3) (`KismetMathLibrary.BreakVector` (`SceneComponent.K2_GetComponentLocation` (`self.WalkablePlatform`))))
  (`SceneComponent.K2_SetWorldLocation` (`self.MirorPlatform`) (`KismetMathLibrary.MakeVector` _returnvalue_x_3 _returnvalue_y_3 (- _returnvalue_z (* (- _returnvalue_z_2 _returnvalue_z) DistanceMultiplier))) false false))

(fn `UpdateVerticalMirrorPosition`
  (params (Axis :type "Actor Object Reference") (DistanceMultiplier :type "Float (double-precision)"))
  (bind _returnvalue_x (`KismetMathLibrary.BreakVector` (`self.K2_GetActorLocation` Axis)))
  (bind _returnvalue_x_2 (`KismetMathLibrary.BreakVector` (`self.K2_GetActorLocation`)))
  (bind (_returnvalue_x_3 _returnvalue_y _returnvalue_z) (`KismetMathLibrary.BreakVector` (`SceneComponent.K2_GetComponentLocation` (`self.WalkablePlatform`))))
  (`SceneComponent.K2_SetWorldLocation` (`self.MirorPlatform`) (`KismetMathLibrary.MakeVector` (- _returnvalue_x (* (- _returnvalue_x_2 _returnvalue_x) DistanceMultiplier)) _returnvalue_y _returnvalue_z) false false))

(fn `UserConstructionScript`)