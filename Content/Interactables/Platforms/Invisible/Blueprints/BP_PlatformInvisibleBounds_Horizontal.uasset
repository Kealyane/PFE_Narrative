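; Horizontal bounds Blueprint for invisible platforms, acting as the mirror axis for their reflected positions.
; On BeginPlay it applies its DistanceMult through SetDistanceMult.
; UpdateAllMirrorPlatforms has each listed invisible platform recompute its horizontal mirror position against this actor and multiplier.
; ShowMirrorForOthers draws debug spheres where other listed actors would mirror, reflecting their Z across this actor's height scaled by DistanceMult.
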(event `self.ReceiveBeginPlay`
  (`self.SetDistanceMult` (`self.DistanceMult`)))

(event `self.ReceiveActorBeginOverlap`
  (params (OtherActor :type "Actor Object Reference")))

(event `self.SparkleCollider.OnComponentBeginOverlap`
  (params (OverlappedComponent :type "PrimitiveComponent Object Reference") (OtherActor :type "Actor Object Reference") (OtherComp :type "PrimitiveComponent Object Reference") (OtherBodyIndex :type Integer) (bFromSweep :type Boolean) (SweepResult :type "HitResult Structure (by ref)")))

(fn `ShowMirrorForOthers`
  (bind (_returnvalue_x _returnvalue_y _returnvalue_z) (`KismetMathLibrary.BreakVector` (`self.K2_GetActorLocation`)))
  (for _array_element (`self.OtherPlatformsType`)
    (`/Engine/EditorBlueprintResources/StandardMacros.IsValid` _array_element
      (:`Is Valid`
        (bind (_returnvalue_x_2 _returnvalue_y_2 _returnvalue_z_2) (`KismetMathLibrary.BreakVector` (`self.K2_GetActorLocation` _array_element)))
        (`KismetSystemLibrary.DrawDebugSphere` (`KismetMathLibrary.MakeVector` _returnvalue_x_2 _returnvalue_y_2 (- _returnvalue_z (* (- _returnvalue_z_2 _returnvalue_z) (`self.DistanceMult`)))) 20.0 12 (struct :`R` 1.0 :`G` 0.901434 :`A` 1.0) 120.0 10.0)))))

(fn `UpdateAllMirrorPlatforms`
  (for _array_element (`self.AllInvisiblePlatforms`)
    (`/Engine/EditorBlueprintResources/StandardMacros.IsValid` _array_element
      (:`Is Valid`
        (`/Game/Interactables/Platforms/Invisible/Blueprints/BP_PlatformInvisible.UpdateHorizontalMirrorPosition` _array_element self (`self.DistanceMult`))))))

(fn `UserConstructionScript`)