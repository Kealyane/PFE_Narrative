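; Switchable platform Blueprint that shows its open or closed state by swapping the sprite on its render component.
; On BeginPlay it binds to a status-changed event and sets the initial sprite from AtStartIsOpen.
; When the event fires, it compares the reported platform with itself and changes sprite only for its own state changes.
; The graph handles visuals only, with no state-switching logic of its own.
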(event `self.ReceiveBeginPlay`
  (bind _rendercomponent (`self.RenderComponent`))
  (add `self.StatusChanged` (delegate `StatusChangeEvent`))
  (if (`self.bAtStartIsOpen`)
    (`PaperSpriteComponent.SetSprite` _rendercomponent "/Game/Interactables/Platforms/SwitchState/Sprites/IMG_0502_Sprite_0.IMG_0502_Sprite_0")
    (else
      (`PaperSpriteComponent.SetSprite` _rendercomponent "/Game/Interactables/Platforms/SwitchState/Sprites/IMG_0501_Sprite_0.IMG_0501_Sprite_0"))))

(event `StatusChangeEvent` :!signature `self.StatusChanged`
  (params (Platform :type "PaperPlatformStateChanging Object Reference") (bIsPlatformOpen :type Boolean))
  (bind _rendercomponent (`self.RenderComponent`))
  (if (== Platform self)
    (if bIsPlatformOpen
      (`PaperSpriteComponent.SetSprite` _rendercomponent "/Game/Interactables/Platforms/SwitchState/Sprites/IMG_0502_Sprite_0.IMG_0502_Sprite_0")
      (else
        (`PaperSpriteComponent.SetSprite` _rendercomponent "/Game/Interactables/Platforms/SwitchState/Sprites/IMG_0501_Sprite_0.IMG_0501_Sprite_0")))))

(fn `UserConstructionScript`)