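; BP_StateChanging_Sound is an actor that plays the platform state-switch sound when the player jumps nearby.
; On BeginPlay it casts player pawn 0 to PFECharacter and binds OnJump to that character's jump delegate.
; Overlap begin and end events with a PFECharacter toggle an IsInRange flag, so each jump plays the SwitchState sound only while the character is inside the actor's overlap area.
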(event `self.ReceiveBeginPlay`
  (bind _aspfecharacter (cast `PFECharacter` (`GameplayStatics.GetPlayerPawn` 0)))
  (add `PFECharacter.JumpDelegate` _aspfecharacter (delegate `OnJump`)))

(event `OnJump`
  (if (`self.IsInRange`)
    (`SoundComponent.PlaySound` (`self.Sound`) "SwitchState")))

(event `self.ReceiveActorBeginOverlap`
  (params (OtherActor :type "Actor Object Reference"))
  (cast `PFECharacter` OtherActor)
  (set `self.IsInRange` true))

(event `self.ReceiveActorEndOverlap`
  (params (OtherActor :type "Actor Object Reference"))
  (cast `PFECharacter` OtherActor)
  (set `self.IsInRange` false))

(fn `UserConstructionScript`)