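; BP_DoorFlame is a 2D sprite door that opens or closes in response to a bound CanDoorOpen notification.
; InitSprites picks the open and closed sprites from DoorType (Small or Medium) and shows the closed one, both at construction and at BeginPlay.
; On each notification it swaps the sprite, plays the matching sound, and switches the box's Pawn collision between Ignore and Block.
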(event `self.ReceiveBeginPlay`
  (add `self.CanDoorOpen` (delegate `OnCanDoorOpen`))
  (`self.InitSprites`))

(event `OnCanDoorOpen` :!signature `self.CanDoorOpen`
  (params (bIsOpen :type Boolean))
  (if bIsOpen
    ;[0.3605 1 0.3974] Door Open
    (`PaperSpriteComponent.SetSprite` (`self.PaperSprite`) (`self.OpenSprite`))
    (`GameplayStatics.PlaySound2D` "/Game/Interactables/Doors/Sounds/DoorSound_Cue.DoorSound_Cue" 1.0 1.0 0.0 null null)
    (`PrimitiveComponent.SetCollisionResponseToChannel` (`self.Box`) "ECC_Pawn" "ECR_Ignore")
    (else
      ;[1 0.3405 0.3227] Door Close
      (`PaperSpriteComponent.SetSprite` (`self.PaperSprite`) (`self.CloseSprite`))
      (`GameplayStatics.PlaySound2D` "/Game/Interactables/Doors/Sounds/DoorCloseSound_Cue.DoorCloseSound_Cue" 1.0 1.0 0.0 null null)
      (`PrimitiveComponent.SetCollisionResponseToChannel` (`self.Box`) "ECC_Pawn" "ECR_Block"))))

(fn `InitSprites`
  (switch `EIntensity` (`self.DoorType`)
    (:`Small`
      (set `self.OpenSprite` "/Game/Interactables/Doors/Sprites/Porte_04Open_Sprite_0.Porte_04Open_Sprite_0")
      (bind _output_get (set `self.CloseSprite` "/Game/Interactables/Doors/Sprites/Porte_04_BW_Sprite_0.Porte_04_BW_Sprite_0"))
      (`PaperSpriteComponent.SetSprite` (`self.PaperSprite`) _output_get))
    (:`Medium`
      (set `self.OpenSprite` "/Game/Interactables/Doors/Sprites/Porte_03Open_Sprite_0.Porte_03Open_Sprite_0")
      (bind _output_get_2 (set `self.CloseSprite` "/Game/Interactables/Doors/Sprites/Porte_03BW_Sprite_0.Porte_03BW_Sprite_0"))
      (`PaperSpriteComponent.SetSprite` (`self.PaperSprite`) _output_get_2))))

(fn `UserConstructionScript`
  (`self.InitSprites`))