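; BP_DoorKey is a sprite-based door, in Normal or Trapped style, that blocks with a box until opened.
; InitSprite picks the open and closed sprites from DoorType and shows the closed one, running at construction and BeginPlay.
; BeginPlay also binds OnOpenDoor to an open-door delegate; when fired, it plays a 2D sound, shows the open sprite and disables box collision.
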(event `self.ReceiveBeginPlay`
  (`self.InitSprite`)
  (add `self.OpenDoorDelegate` (delegate `OnOpenDoor`)))

(event `OnOpenDoor`
  (`GameplayStatics.PlaySound2D` "/Game/Interactables/Doors/Sounds/DoorSound_Cue.DoorSound_Cue" 1.0 1.0 0.0 null null)
  (`PaperSpriteComponent.SetSprite` (`self.Sprite`) (`self.OpenSprite`))
  (`PrimitiveComponent.SetCollisionEnabled` (`self.Box`) "NoCollision"))

(fn `InitSprite`
  (switch `EDoorKeyType` (`self.DoorType`)
    (:`Normal`
      (set `self.OpenSprite` "/Game/Interactables/Doors/Sprites/Portes_Key-2_Sprite_0.Portes_Key-2_Sprite_0")
      (bind _output_get (set `self.CloseSprite` "/Game/Interactables/Doors/Sprites/Portes_Key-1_Sprite_0.Portes_Key-1_Sprite_0"))
      (`PaperSpriteComponent.SetSprite` (`self.Sprite`) _output_get))
    (:`Trapped`
      (set `self.OpenSprite` "/Game/Interactables/Doors/Sprites/trapdoor_open_Sprite_0.trapdoor_open_Sprite_0")
      (bind _output_get_2 (set `self.CloseSprite` "/Game/Interactables/Doors/Sprites/trapdoor_closed_Sprite_0.trapdoor_closed_Sprite_0"))
      (`PaperSpriteComponent.SetSprite` (`self.Sprite`) _output_get_2))))

(fn `UserConstructionScript`
  (`self.InitSprite`))