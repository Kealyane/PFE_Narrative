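; BP_DoorSimple is a sprite-based door that closes behind the player once they exit on a configured side.
; On end overlap, an open door compares the player capsule's world X with a sphere position cached at BeginPlay, using ExitOnTheRight to choose the side.
; Close plays a sound, then after a short delay swaps to the closed sprite, restores collision and clears DoorIsOpen.
; Separate events swap the open and closed sprites without changing state.
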(event `self.ReceiveBeginPlay`
  (set `self.RefPosition` (`SceneComponent.K2_GetComponentLocation` (`self.Sphere`))))

(event `self.ReceiveActorEndOverlap`
  (params (OtherActor :type "Actor Object Reference"))
  (bind _refposition_x (`KismetMathLibrary.BreakVector` (`self.RefPosition`)))
  (bind _refposition_x_2 (`KismetMathLibrary.BreakVector` (`self.RefPosition`)))
  (if (`self.DoorIsOpen`)
    (bind _asbp_player (cast `/Game/Characters/Player/Blueprints/BP_Player` OtherActor))
    (if (`self.ExitOnTheRight`)
      (bind _returnvalue_x (`KismetMathLibrary.BreakVector` (`SceneComponent.K2_GetComponentLocation` (`Character.CapsuleComponent` _asbp_player))))
      (if (< _refposition_x_2 _returnvalue_x)
        (`self.Close`))
      (else
        (bind _returnvalue_x_2 (`KismetMathLibrary.BreakVector` (`SceneComponent.K2_GetComponentLocation` (`Character.CapsuleComponent` _asbp_player))))
        (if (> _refposition_x _returnvalue_x_2)
          (`self.Close`))))))

(event `Close`
  (bind _audio (`self.Audio`))
  (`AudioComponent.SetSound` _audio "/Game/Interactables/Doors/Sounds/DoorCloseSound_Cue.DoorCloseSound_Cue")
  (`AudioComponent.Play` _audio 0.0)
  (`KismetSystemLibrary.Delay` 0.3)
  (`PaperSpriteComponent.SetSprite` (`self.Door`) "/Game/Interactables/Doors/Sprites/PorteFermee_Sprite.PorteFermee_Sprite")
  (`PrimitiveComponent.SetCollisionEnabled` (`self.Collider`) "QueryAndPhysics")
  (set `self.DoorIsOpen` false))

(event `ChangeMeshToOpen`
  (`PaperSpriteComponent.SetSprite` (`self.Door`) "/Game/Interactables/Doors/Sprites/PorteOuverte_Sprite.PorteOuverte_Sprite"))

(event `ChangeMeshToClosed`
  (`PaperSpriteComponent.SetSprite` (`self.Door`) "/Game/Interactables/Doors/Sprites/PorteFermee_Sprite.PorteFermee_Sprite"))

(fn `UserConstructionScript`)