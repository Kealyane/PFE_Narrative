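; BP_SmallFlameDoorV2 is a small sprite door that opens once enough flames are activated.
; BeginPlay creates a BP_DoorCounter widget, flags it as a small door and seeds its flame counts.
; CheckFlames refreshes the counter slider and compares activated to required flames, toggling sprite and collision between blocking and overlap, with a sound when open.
; The nodes for attaching the widget and toggling visibility are disconnected.
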(event `self.ReceiveBeginPlay`
  (set `self.ActivatedFlames` 0)
  (bind _returnvalue (`|CreateWidget` "/Game/Prototype/Blueprints/Doors/BP_DoorCounter.BP_DoorCounter_C"))
  (set `self.DoorCounter` _returnvalue)
  (set `/Game/Prototype/Blueprints/Doors/BP_DoorCounter.TotalFlames` (`KismetMathLibrary.Conv_IntToDouble` (`self.NumberOfFlames`)) _returnvalue)
  (set `/Game/Prototype/Blueprints/Doors/BP_DoorCounter.CurrentFlames` (`KismetMathLibrary.Conv_IntToDouble` (`self.ActivatedFlames`)) _returnvalue)
  (set `/Game/Prototype/Blueprints/Doors/BP_DoorCounter.IsSmallDoor` true _returnvalue)
  (`/Game/Prototype/Blueprints/Doors/BP_DoorCounter.CheckSliderColor` _returnvalue))

(event `CheckFlamesForWidget`
  (bind _doorcounter (`self.DoorCounter`))
  (set `/Game/Prototype/Blueprints/Doors/BP_DoorCounter.TotalFlames` (`KismetMathLibrary.Conv_IntToDouble` (`self.NumberOfFlames`)) _doorcounter)
  (set `/Game/Prototype/Blueprints/Doors/BP_DoorCounter.CurrentFlames` (`KismetMathLibrary.Conv_IntToDouble` (`self.ActivatedFlames`)) _doorcounter))

(event `CheckFlames`
  (`self.CheckFlamesForWidget`)
  (`/Game/Prototype/Blueprints/Doors/BP_DoorCounter.SetSlider` (`self.DoorCounter`))
  (if (> (`self.NumberOfFlames`) (`self.ActivatedFlames`))
    (`PaperSpriteComponent.SetSprite` (`self.Door`) "/Game/Interactables/Doors/Sprites/Porte_04_BW_Sprite_0.Porte_04_BW_Sprite_0")
    (`PrimitiveComponent.SetCollisionResponseToAllChannels` (`self.Collider`) "ECR_Block")
    (else
      (`PaperSpriteComponent.SetSprite` (`self.Door`) "/Game/Interactables/Doors/Sprites/Porte_04Open_Sprite_0.Porte_04Open_Sprite_0")
      (`PrimitiveComponent.SetCollisionResponseToAllChannels` (`self.Collider`) "ECR_Overlap")
      (`GameplayStatics.PlaySoundAtLocation` "/Game/Interactables/Doors/Sounds/DoorSound_Cue.DoorSound_Cue" (`SceneComponent.K2_GetComponentLocation` (`self.DefaultSceneRoot`)) (struct) 1.0 1.0 0.0 null null null null))))

(fn `UserConstructionScript`)