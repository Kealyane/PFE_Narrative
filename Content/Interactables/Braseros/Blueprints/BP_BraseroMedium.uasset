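; Medium brasero (brazier) interactable that gives sound and visual feedback when it is lit, put out or given a wrong flame.
; BeginPlay sets its unique ID and assigns handlers for turn on, turn off, small wrong flame and big wrong flame.
; A small wrong flame briefly shows a flipbook, while a big one plays an explosion sound, hides the brasero and explosion flipbook on timed delays, then restores the brasero.
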(event `self.ReceiveBeginPlay`
  (`self.SetUniqueIDComp` (`self.UniqueID`))
  (add `self.TurnOnEvent` (delegate `OnTurnOn`))
  (add `self.TurnOffEvent` (delegate `OnTurnOff`))
  (add `self.WrongFlameSmallEvent` (delegate `OnWrongFlameSmall`))
  (add `self.WrongFlameBigEvent` (delegate `OnWrongFlameBig`)))

(event `OnTurnOn`
  (`GameplayStatics.PlaySound2D` "/Game/Interactables/Braseros/Sounds/SC_BraseroLit.SC_BraseroLit" 1.0 1.0 0.0 null null))

(event `OnTurnOff`
  (`GameplayStatics.PlaySound2D` "/Game/Interactables/Braseros/Sounds/SC_BraseroOut.SC_BraseroOut" 1.0 1.0 0.0 null null))

(event `OnWrongFlameSmall`
  (`GameplayStatics.PlaySound2D` "/Game/Interactables/Braseros/Sounds/WrongFlame_Cue.WrongFlame_Cue" 1.0 1.0 0.0 null null)
  (`SceneComponent.SetHiddenInGame` (`self.Wrong Flame Flipbook`) false false)
  (`KismetSystemLibrary.Delay` 0.4)
  (`SceneComponent.SetHiddenInGame` (`self.Wrong Flame Flipbook`) true false))

(event `OnWrongFlameBig`
  (`GameplayStatics.PlaySound2D` "/Game/Interactables/Braseros/Sounds/SC_BraseroExploded.SC_BraseroExploded" 1.0 1.0 0.0 null null)
  (`KismetSystemLibrary.Delay` 0.2)
  (`self.HideBrasero` true)
  (`KismetSystemLibrary.Delay` 0.8)
  (`SceneComponent.SetHiddenInGame` (`self.ExplosionFlipbook`) true false)
  (`KismetSystemLibrary.Delay` 2.0)
  (`self.HideBrasero` false))

(fn `UserConstructionScript`)