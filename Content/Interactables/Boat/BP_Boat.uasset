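; Boat interactable that carries the player on a one-way scripted ride presented as a cinematic.
; When the player enters Detection, a Timeline starts; leaving stops it and re-arms the trigger.
; Once the Timeline finishes, input switches to UI-only, the blocker drops, InterpToMovement starts, and boat sound and cinematic widget play.
; When movement stops, sound fades, the widget animation is uncalled, and ReachedEnd prevents retriggering.
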(event `self.ReceiveBeginPlay`)

(event `self.Detection.OnComponentBeginOverlap`
  (params (OverlappedComponent :type "PrimitiveComponent Object Reference") (OtherActor :type "Actor Object Reference") (OtherComp :type "PrimitiveComponent Object Reference") (OtherBodyIndex :type Integer) (bFromSweep :type Boolean) (SweepResult :type "HitResult Structure (by ref)"))
  (cast `PFECharacter` OtherActor)
  (`/Engine/EditorBlueprintResources/StandardMacros.DoOnce` false :!label _label
    (:`Completed`
      (if (not (`self.ReachedEnd`))
        (set `self.PlayerIn` true)
        (`Timeline|Timeline` :!via `PlayFromStart` :!label _label_2
          (:`Finished`
            (if (`self.PlayerIn`)
              (`WidgetBlueprintLibrary.SetInputMode_UIOnlyEx` (`GameplayStatics.GetPlayerController` 0) null "DoNotLock" true)
              (`KismetSystemLibrary.Delay` 0.2)
              (`PrimitiveComponent.SetCollisionEnabled` (`self.Blocker`) "NoCollision")
              (`ActorComponent.Activate` (`self.InterpToMovement`) false)
              (`SoundComponent.PlaySound` (`self.Sound`) "Boat")
              (`/Engine/EditorBlueprintResources/StandardMacros.DoOnce` false
                (:`Completed`
                  (bind _returnvalue (`|CreateWidget` "/Game/UI/Widgets/Cinematic/WBP_Cinematic.WBP_Cinematic_C"))
                  (bind _output_get (set `self.Widget` _returnvalue))
                  (`UserWidget.AddToViewport` _output_get 0)
                  (`/Game/UI/Widgets/Cinematic/WBP_Cinematic.CallAnimNoZoom` _output_get))))))))))

(event `Stop`
  (goto _label_2 :!via `Stop`))

(event `Reboot`
  (goto _label :!via `Reset`))

(event `self.InterpToMovement.OnInterpToStop`
  (params (ImpactResult :type "HitResult Structure (by ref)") (Time :type "Float (single-precision)"))
  (`SoundComponent.StopSmoothSound` (`self.Sound`) 0.5)
  (`/Game/UI/Widgets/Cinematic/WBP_Cinematic.UncallAnimNoZoom` (`self.Widget`))
  (set `self.ReachedEnd` true))

(event `self.Detection.OnComponentEndOverlap`
  (params (OverlappedComponent :type "PrimitiveComponent Object Reference") (OtherActor :type "Actor Object Reference") (OtherComp :type "PrimitiveComponent Object Reference") (OtherBodyIndex :type Integer))
  (`self.Stop`)
  (set `self.PlayerIn` false)
  (`self.Reboot`))

(fn `UserConstructionScript`)