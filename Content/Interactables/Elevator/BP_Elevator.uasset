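; One-way elevator that carries the player once they step into its trigger and are still inside when a timeline finishes.
; It then makes the left and right blockers block Pawns, activates InterpToMovement and plays lift sounds through one audio component.
; A DoOnce guards boarding and re-arms if the trigger is exited before arrival.
; When movement stops, it marks arrival, releases the blockers through a timer-driven check and fades out the audio.
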(event `self.ReceiveBeginPlay`)

(event `self.Trigger.OnComponentBeginOverlap`
  (params (OverlappedComponent :type "PrimitiveComponent Object Reference") (OtherActor :type "Actor Object Reference") (OtherComp :type "PrimitiveComponent Object Reference") (OtherBodyIndex :type Integer) (bFromSweep :type Boolean) (SweepResult :type "HitResult Structure (by ref)"))
  (`/Engine/EditorBlueprintResources/StandardMacros.DoOnce` false :!label _label
    (:`Completed`
      (if (not (`self.HasArrived`))
        (cast `PFECharacter` OtherActor)
        (set `self.PlayerIn` true)
        (`Timeline|Timeline` :!via `PlayFromStart` :!label _label_2
          (:`Finished`
            (if (`self.PlayerIn`)
              (`self.ActiveBlocker` true)
              (`self.PlaySound` "/Game/Sounds/Lift/LiftStart_Cue.LiftStart_Cue")
              (`ActorComponent.Activate` (`self.InterpToMovement`) false)
              (`self.PlaySound` "/Game/Sounds/Lift/LiftLoop_Cue.LiftLoop_Cue"))))))))

(event `Reboot`
  (goto _label :!via `Reset`))

(event `Reset`
  (goto _label_2 :!via `Stop`))

(event `self.InterpToMovement.OnInterpToStop`
  (params (ImpactResult :type "HitResult Structure (by ref)") (Time :type "Float (single-precision)"))
  (set `self.HasArrived` true)
  (`self.CheckCollisions`)
  (`AudioComponent.FadeOut` (`self.Audio`) 0.2 0.0 "Linear")
  (`KismetSystemLibrary.Delay` 0.5)
  (if (`AudioComponent.IsPlaying` (`self.Audio`))
    (`AudioComponent.FadeOut` (`self.Audio`) 0.2 0.0 "Linear")))

(event `self.Trigger.OnComponentEndOverlap`
  (params (OverlappedComponent :type "PrimitiveComponent Object Reference") (OtherActor :type "Actor Object Reference") (OtherComp :type "PrimitiveComponent Object Reference") (OtherBodyIndex :type Integer))
  (set `self.PlayerIn` false)
  (if (not (`self.HasArrived`))
    (`self.Reboot`)))

(event `CheckCollisions`
  (bind _returnvalue (`KismetSystemLibrary.K2_SetTimerDelegate` (delegate `CheckCollisions`) 0.1 true))
  (if (`self.HasArrived`)
    (`self.ActiveBlocker` false)
    (`KismetSystemLibrary.Delay` 1.0)
    (`KismetSystemLibrary.K2_ClearAndInvalidateTimerHandle` _returnvalue)))

(fn `ActiveBlocker`
  (params (Enable :type Boolean))
  (if Enable
    (`PrimitiveComponent.SetCollisionResponseToChannel` (`self.BlockerRight`) "ECC_Pawn" "ECR_Block")
    (`PrimitiveComponent.SetCollisionResponseToChannel` (`self.BlockerLeft`) "ECC_Pawn" "ECR_Block")
    (else
      (`PrimitiveComponent.SetCollisionResponseToChannel` (`self.BlockerRight`) "ECC_Pawn" "ECR_Ignore")
      (`PrimitiveComponent.SetCollisionResponseToChannel` (`self.BlockerLeft`) "ECC_Pawn" "ECR_Ignore"))))

(fn `PlaySound`
  (params (SFX :type "SoundCue Object Reference"))
  (bind _audio (`self.Audio`))
  (`AudioComponent.Stop` _audio)
  (`AudioComponent.SetSound` _audio SFX)
  (`AudioComponent.Play` _audio 0.0))

(fn `UserConstructionScript`)