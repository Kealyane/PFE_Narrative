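; BP_NewBoss is a flipbook-animated boss that exposes events for walking, idling and yelling.
; Yell plays a sound and sets WasShoved on the player, StopYell clears it, and MakeFlamesAppear forwards to BP_Player.
; WalkLeft and WalkRight both use the BossWalkRight flipbook, with no flip in these events.
; Insult is empty, and the insult bubble visibility calls are disconnected.
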(event `WalkLeft`
  (`PaperFlipbookComponent.SetFlipbook` (`self.PaperFlipbook`) "/Game/Characters/Boss/Flipbooks/BossWalkRight.BossWalkRight"))

(event `WalkRight`
  (`PaperFlipbookComponent.SetFlipbook` (`self.PaperFlipbook`) "/Game/Characters/Boss/Flipbooks/BossWalkRight.BossWalkRight"))

(event `Yell`
  (`PaperFlipbookComponent.SetFlipbook` (`self.PaperFlipbook`) "/Game/Characters/Boss/Flipbooks/BossYell.BossYell")
  (`GameplayStatics.PlaySoundAtLocation` "/Game/Characters/Boss/Sounds/AngruBoss_Cue.AngruBoss_Cue" (`SceneComponent.K2_GetComponentLocation` (`self.PaperFlipbook`)) (struct) 1.0 1.0 0.0 null null null null)
  (bind _asbp_player (cast `/Game/Characters/Player/Blueprints/BP_Player` (`GameplayStatics.GetPlayerCharacter` 0)))
  (set `/Game/Characters/Player/Blueprints/BP_Player.WasShoved` true _asbp_player))

(event `Idle`
  (`PaperFlipbookComponent.SetFlipbook` (`self.PaperFlipbook`) "/Game/Characters/Boss/Flipbooks/BossIdle.BossIdle"))

(event `Insult`)

(event `StopYell`
  (bind _asbp_player (cast `/Game/Characters/Player/Blueprints/BP_Player` (`GameplayStatics.GetPlayerCharacter` 0)))
  (set `/Game/Characters/Player/Blueprints/BP_Player.WasShoved` false _asbp_player))

(event `MakeFlamesAppear`
  (bind _returnvalue (`GameplayStatics.GetActorOfClass` "/Game/Characters/Player/Blueprints/BP_Player.BP_Player_C"))
  (`/Game/Characters/Player/Blueprints/BP_Player.MakeFlamesAppear` _returnvalue))

(fn `UserConstructionScript`)