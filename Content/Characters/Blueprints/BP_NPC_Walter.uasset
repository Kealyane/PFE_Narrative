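; Walter NPC Blueprint that either stays idle or patrols back and forth between two preset locations.
; A self-repeating Move event slides the capsule to each location with MoveComponentTo over a set time, pauses briefly, then alternates the target index.
; Each leg starts with a 180-degree yaw flip, except the first, which flips conditionally based on an X-position comparison.
; An IsMoving flag tracks when it is travelling.
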(event `self.ReceiveBeginPlay`
  (if (not (`self.StaysIdle`))
    (set `self.InitRot` (`SceneComponent.K2_GetComponentRotation` (`self.CapsuleComponent`)))
    (`self.Move`)))

(event `Move`
  (bind _capsulecomponent (`self.CapsuleComponent`))
  (bind _capsulecomponent_2 (`self.CapsuleComponent`))
  (bind (_returnvalue_roll _returnvalue_pitch _returnvalue_yaw) (`KismetMathLibrary.BreakRotator` (`SceneComponent.K2_GetComponentRotation` _capsulecomponent)))
  (bind (_returnvalue_roll_2 _returnvalue_pitch_2 _returnvalue_yaw_2) (`KismetMathLibrary.BreakRotator` (`SceneComponent.K2_GetComponentRotation` _capsulecomponent_2)))
  (bind _returnvalue_x (`KismetMathLibrary.BreakVector` (`SceneComponent.K2_GetComponentLocation` (`self.CapsuleComponent`))))
  (bind _output_x (`KismetMathLibrary.BreakVector` (`|GetArrayItem` (`self.Location`) (`self.Locations`))))
  (`|ExecutionSequence`
    (:`then_0`
      (if (`self.FirstRun`)
        (set `self.FirstRun` false)
        (if (not (> _returnvalue_x _output_x))
          (`SceneComponent.K2_SetWorldRotation` _capsulecomponent_2 (`KismetMathLibrary.MakeRotator` 0.0 0.0 (+ _returnvalue_yaw_2 180.0)) false false)
          (set `self.NewRot` (`SceneComponent.K2_GetComponentRotation` (`self.CapsuleComponent`))))
        (else
          (`SceneComponent.K2_SetWorldRotation` _capsulecomponent (`KismetMathLibrary.MakeRotator` 0.0 0.0 (+ _returnvalue_yaw 180.0)) false false)
          (set `self.NewRot` (`SceneComponent.K2_GetComponentRotation` (`self.CapsuleComponent`))))))
    (:`then_1`
      (set `self.IsMoving` true)
      (`KismetSystemLibrary.MoveComponentTo` (`self.CapsuleComponent`) (`|GetArrayItem` (`self.Location`) (`self.Locations`)) (`self.NewRot`) false false (`self.TimeToLoc`))
      (set `self.IsMoving` false)
      (`KismetSystemLibrary.Delay` 1.0)
      (`/Engine/EditorBlueprintResources/StandardMacros.IncrementInt` (`self.Locations`)
        (:`  `
          (if (== (`self.Locations`) 2)
            (set `self.Locations` 0))
          (`self.Move`))))))

(fn `UserConstructionScript`)