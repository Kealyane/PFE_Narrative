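; Player controller that mounts the root UI, tracks the active input device and relays UI key presses.
; BeginPlay adds the GameInstance's root widget to the viewport, creating it if missing, and binds CommonInput method changes, which update gamepad flags and notify listeners.
; Back, debug and pause keys fire events, with Tab pausing only in editor.
; Helper functions open and close the pause menu, toggle player movement and restore the saved input type.
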(event `self.ReceiveBeginPlay`
  ;[1 1 1] Init
  (add `CommonInputSubsystem.OnInputMethodChanged` (subsystem `CommonInputSubsystem`) (`|CreateDelegate` :!event `OnInputChange`))
  (bind _asbp_pfegame_instance (cast `/Game/Blueprints/Core/BP_PFEGameInstance` (`GameplayStatics.GetGameInstance`)))
  (bind _output_get (set `self.MyGameInstance` _asbp_pfegame_instance))
  (bind _widgetroot (`/Game/Blueprints/Core/BP_PFEGameInstance.WidgetRoot` _output_get))
  (`/Engine/EditorBlueprintResources/StandardMacros.IsValid` _widgetroot
    (:`Is Valid`
      (`UserWidget.AddToViewport` _widgetroot 0)
      (`self.UIAddedToViewportEvent`))
    (:`Is Not Valid`
      (bind _returnvalue (`|CreateWidget` "/Game/UI/Widgets/Menus/NewWay/WBP_Root.WBP_Root_C"))
      (bind _output_get_2 (set `/Game/Blueprints/Core/BP_PFEGameInstance.WidgetRoot` _returnvalue (`self.MyGameInstance`)))
      (`UserWidget.AddToViewport` _output_get_2 0)
      (`self.UIAddedToViewportEvent`))))

(event `OnInputChange`
  (params (bNewInputType :type "ECommonInputType Enum" :default "MouseAndKeyboard"))
  ;[1 1 1] Input Change
  (`self.OnInputControllerChanged` bNewInputType)
  (switch `ECommonInputType` bNewInputType
    (:`MouseAndKeyboard`
      (set `self.IsGamepadController` false)
      (set `/Game/Blueprints/Core/BP_PFEGameInstance.IsGamepad` false (`self.MyGameInstance`))
      (`KismetSystemLibrary.PrintString` "PC::OnInputChange = keyboard" true true (struct :`G` 0.66 :`B` 1.0 :`A` 1.0) 5.0))
    (:`Gamepad`
      (set `self.IsGamepadController` true)
      (set `/Game/Blueprints/Core/BP_PFEGameInstance.IsGamepad` true (`self.MyGameInstance`))
      (`KismetSystemLibrary.PrintString` "PC::OnInputChange = gamepad" true true (struct :`G` 0.66 :`B` 1.0 :`A` 1.0) 5.0))))

(event `Key|Gamepad_FaceButton_Right`
  (params (Key :type "Key Structure"))
  ;[1 1 1] UI Back Input
  (:`Pressed`
    (`self.GamepadBackPressedEvent`)))

(event `Key|Equals`
  (params (Key :type "Key Structure"))
  ;[1 1 1] UI Debug Input
  (:`Pressed`
    (`self.DebugMenuPressedEvent` :!label _label)))

(event `Key|Gamepad_LeftShoulder`
  (params (Key :type "Key Structure"))
  ;[1 1 1] UI Debug Input
  (:`Pressed`
    (goto _label)))

(event `Key|Tab`
  (params (Key :type "Key Structure"))
  ;[1 1 1] UI Pause Input
  (:`Pressed`
    (if (`PFEEditorUtility.IsEditor`)
      (`self.PauseMenuPressedEvent` :!label _label_2))))

(event `Key|Escape`
  (params (Key :type "Key Structure"))
  ;[1 1 1] UI Pause Input
  (:`Pressed`
    (goto _label_2)))

(event `Key|Gamepad_Special_Right`
  (params (Key :type "Key Structure"))
  ;[1 1 1] UI Pause Input
  (:`Pressed`
    (goto _label_2)))

(fn `CreateMenu`
  (bind _returnvalue (`|CreateWidget` "/Game/UI/Widgets/Menus/CWBP_PauseMenu.CWBP_PauseMenu_C"))
  (bind _output_get (set `self.CommonPauseMenu` _returnvalue))
  (`UserWidget.AddToViewport` _output_get 0)
  (set `self.IsPauseOpen` true)
  (`WidgetBlueprintLibrary.SetInputMode_GameAndUIEx` self null "DoNotLock" false))

(fn `DisableGameInput`
  (bind _asbp_player (cast `/Game/Characters/Player/Blueprints/BP_Player` (`GameplayStatics.GetPlayerCharacter` 0)))
  (set `PFECharacter.bCanMove` false _asbp_player))

(fn `EnableGameInput`
  (bind _asbp_player (cast `/Game/Characters/Player/Blueprints/BP_Player` (`GameplayStatics.GetPlayerCharacter` 0)))
  (set `PFECharacter.bCanMove` true _asbp_player))

(fn `IsGamepad`
  (returns (IsGamepad :type Boolean))
  (bind (_returnvalue_inputclassname _returnvalue_hardwaredeviceidentifier _returnvalue_primarydevicetype) (break `HardwareDeviceIdentifier` (`InputDeviceSubsystem.GetMostRecentlyUsedHardwareDevice` :`self` (subsystem `InputDeviceSubsystem`))))
  (switch `EHardwareDevicePrimaryType` _returnvalue_primarydevicetype
    (:`KeyboardAndMouse`
      (`KismetSystemLibrary.PrintString` "PC::IsGamepad NO keyboard and mouse" true true (struct :`G` 0.66 :`B` 1.0 :`A` 1.0) 5.0)
      (return false))
    (:`Gamepad`
      (`KismetSystemLibrary.PrintString` "PC::IsGamepad YES" true true (struct :`G` 0.66 :`B` 1.0 :`A` 1.0) 5.0)
      (return true))))

(fn `RemoveMenu`
  (`KismetSystemLibrary.PrintString` "PC::RemoveMenu" true true (struct :`R` 1.0 :`G` 0.964141 :`B` 0.224174 :`A` 1.0) 10.0)
  (`Widget.RemoveFromParent` (`self.CommonPauseMenu`))
  (`WidgetBlueprintLibrary.SetInputMode_GameOnly` self)
  (set `self.bShowMouseCursor` false)
  (`self.EnableGameInput`)
  (set `self.IsPauseOpen` false))

(fn `SetController`
  (params (In_BP_PFE_GameInstance :type "/Game/Blueprints/Core/BP_PFEGameInstance Object Reference"))
  (bind _returnvalue (subsystem `CommonInputSubsystem`))
  (`KismetSystemLibrary.PrintString` "PC::Set Controller" true true (struct :`G` 0.66 :`B` 1.0 :`A` 1.0) 10.0)
  (if (`/Game/Blueprints/Core/BP_PFEGameInstance.IsGamepad` In_BP_PFE_GameInstance)
    (`CommonInputSubsystem.SetCurrentInputType` _returnvalue "Gamepad")
    (else
      (`CommonInputSubsystem.SetCurrentInputType` _returnvalue "MouseAndKeyboard")))
  (`KismetSystemLibrary.PrintString` (`|GetEnumeratorNameAsString` (`CommonInputSubsystem.GetCurrentInputType` _returnvalue)) true true (struct :`G` 0.66 :`B` 1.0 :`A` 1.0) 10.0))

(fn `SetUserFocusWidget`
  (params (Button :type "UserWidget Object Reference"))
  (return))

(fn `UserConstructionScript`)