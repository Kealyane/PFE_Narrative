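; Player character: a sprite-based flame whose small, normal and high states swap animation Blueprint, light and post-process sphere scale.
; BeginPlay wires up the C++ movement, wall-detection, flame and sound components, whose delegates drive those states, smoke and wall-grab sprite offset.
; Tick orients scene-capture reflections by move direction, eases camera look-ahead and pulses sprite color in flame-changing zones.
; Also holds cinematic pose events and editor-only flame debug keys.
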(event `Key|S`
  (params (Key :type "Key Structure"))
  (:`Pressed`
    (if (`PFEEditorUtility.IsEditor`)
      (`FlameComponent.SetFlameValue` (`self.Flame`) 29.0))))

(event `Key|M`
  (params (Key :type "Key Structure"))
  (:`Pressed`
    (if (`PFEEditorUtility.IsEditor`)
      (`FlameComponent.SetFlameValue` (`self.Flame`) 50.0))))

(event `Key|B`
  (params (Key :type "Key Structure"))
  (:`Pressed`
    (if (`PFEEditorUtility.IsEditor`)
      (`FlameComponent.SetFlameValue` (`self.Flame`) 71.0))))

(event `SetAnimToSmall`
  (bind _playerlight (`self.PlayerLight`))
  ;[1 1 1] SetAnimFlame
  (`/Engine/EditorBlueprintResources/StandardMacros.DoOnce` false :!label _label
    (:`Completed`
      (`self.ResetDefault`)
      (`self.ResetBig`)
      (`PaperZDAnimationComponent.SetAnimInstanceClass` (`self.AnimationComponent`) "/Game/Characters/Player/Animations/ABP_SmallFlame.ABP_SmallFlame_C")
      (`LightComponent.SetIntensity` _playerlight 8000.0)
      (`LightComponent.SetLightColor` _playerlight (struct :`R` 1.0 :`G` 0.352873 :`B` 0.114305 :`A` 1.0) true)
      (`SceneComponent.SetWorldScale3D` (`self.SpherePostProcess`) (10.0 10.0 16.5)))))

(event `ResetSmall`
  ;[1 1 1] SetAnimFlame
  (goto _label :!via `Reset`))

(event `SetAnimToDefault`
  (bind _playerlight (`self.PlayerLight`))
  ;[1 1 1] SetAnimFlame
  (`/Engine/EditorBlueprintResources/StandardMacros.DoOnce` false :!label _label_2
    (:`Completed`
      (`self.ResetSmall`)
      (`self.ResetBig`)
      (`PaperZDAnimationComponent.SetAnimInstanceClass` (`self.AnimationComponent`) "/Game/Characters/Player/Animations/ABP_MidFlame.ABP_MidFlame_C")
      (`LightComponent.SetIntensity` _playerlight 10000.0)
      (`LightComponent.SetLightColor` _playerlight (struct :`R` 1.0 :`G` 0.610227 :`B` 0.228658 :`A` 1.0) true)
      (`SceneComponent.SetWorldScale3D` (`self.SpherePostProcess`) (15.0 15.0 23.0)))))

(event `ResetDefault`
  ;[1 1 1] SetAnimFlame
  (goto _label_2 :!via `Reset`))

(event `SetAnimToBig`
  (bind _playerlight (`self.PlayerLight`))
  ;[1 1 1] SetAnimFlame
  (`/Engine/EditorBlueprintResources/StandardMacros.DoOnce` false :!label _label_3
    (:`Completed`
      (`self.ResetSmall`)
      (`self.ResetDefault`)
      (`PaperZDAnimationComponent.SetAnimInstanceClass` (`self.AnimationComponent`) "/Game/Characters/Player/Animations/ABP_BigFlame.ABP_BigFlame_C")
      (`LightComponent.SetIntensity` _playerlight 20000.0)
      (`LightComponent.SetLightColor` _playerlight (struct :`R` 1.0 :`G` 0.798585 :`B` 0.241234 :`A` 1.0) true)
      (`SceneComponent.SetWorldScale3D` (`self.SpherePostProcess`) (20.0 20.0 28.0)))))

(event `ResetBig`
  ;[1 1 1] SetAnimFlame
  (goto _label_3 :!via `Reset`))

(event `self.ReceiveBeginPlay`
  (`|ExecutionSequence`
    (:`then_0`
      ;[0.3884 0.6751 1] Reflexion
      (`SceneCaptureComponent.ShowOnlyComponent` (`self.SceneCapture_Horizontal`) (`self.Sprite`))
      (`self.InitReflexionPlaneHorizontal` (`self.ReflexionHorizontal`))
      ;[0.3884 0.6751 1] Reflexion
      (`SceneCaptureComponent.ShowOnlyComponent` (`self.SceneCapture_Vertical`) (`self.Sprite`))
      (`self.InitReflexionPlaneVertical` (`self.ReflexionVertical`))
      (bind _returnvalue (`GameplayStatics.GetCurrentLevelName` true))
      (if (`KismetStringLibrary.EqualEqual_StrStr` _returnvalue "SPITFIRE_Level")
        (set `self.bCanDetectWall` false)
        (else
          (set `self.bCanDetectWall` true))))
    (:`then_1`
      (bind _returnvalue_2 (`GameplayStatics.GetActorOfClass` "/Game/Blueprints/Cameras/BP_MainCamera.BP_MainCamera_C"))
      (`/Engine/EditorBlueprintResources/StandardMacros.IsValid` _returnvalue_2
        (:`Is Valid`
          (if (`PFECameraComponent.bUseDefaultCamera` (`/Game/Blueprints/Cameras/BP_MainCamera.PFECamera` _returnvalue_2))
            (set `self.CameraInitPos` (`SceneComponent.RelativeLocation` (`self.Camera`)) :!label _label_4)
            (else
              (`ActorComponent.Deactivate` (`self.Camera`)))))
        (:`Is Not Valid`
          (goto _label_4))))
    (:`then_2`
      (`self.InitMovementComponent` (`self.CharacterMovement`))
      (`self.InitCapsuleComponent` (`self.CapsuleWallDetection`))
      (`self.InitFlameComponent` (`self.Flame`))
      (`self.InitSoundComponent` (`self.Sound`))
      (`self.InitSceneCaptureCamera` (`self.SceneCapture_Vertical`) (`self.SceneCapture_Horizontal`))
      ;[1 1 1] InitSmoke
      (`ActorComponent.Deactivate` (`self.Smoke`))
      (set `FlameComponent.CurrentZoneEffect` "NORMAL" (`self.Flame`)))
    (:`then_3`
      (if (`self.AreFlameActive`)
        ;[1 0.9528 0.2773] Change animBP depending on Flame
        (add `FlameComponent.OnSmallFlame` (`self.Flame`) (delegate `SmallFlame`))
        (add `FlameComponent.OnNormalFlame` (`self.Flame`) (delegate `NormalFlame`))
        (add `FlameComponent.OnHighFlame` (`self.Flame`) (delegate `HighFlame`))))
    (:`then_4`
      ;[0.4978 0.4978 0.4978] Smoke
      (add `FlameComponent.OnChangeFlameValue` (`self.Flame`) (delegate `ChangeFlameValue`)))
    (:`then_5`
      (add `self.WallGrabDelegate` (delegate `WallGrabEvent`)))))

(event `MakeFlamesAppear`
  (set `self.PlaceholderCanPlay` true)
  (`KismetSystemLibrary.Delay` 3.0)
  (set `self.PlaceholderCanPlay` false)
  (set `self.AreFlameActive` true)
  (`self.NormalFlame`))

(event `CineTrigger`
  (set `self.AreFlameActive` false)
  (`PaperZDAnimationComponent.SetAnimInstanceClass` (`self.AnimationComponent`) "/Game/Cinematic/EndGame/Player/Animations/ABP_FinalCine.ABP_FinalCine_C"))

(event `SmallFlame`
  ;[1 0.9528 0.2773] Change animBP depending on Flame
  (`self.SetAnimToSmall`))

(event `NormalFlame`
  ;[1 0.9528 0.2773] Change animBP depending on Flame
  (`self.SetAnimToDefault`))

(event `HighFlame`
  ;[1 0.9528 0.2773] Change animBP depending on Flame
  (`self.SetAnimToBig`))

(event `CharaWalking`
  (set `self.Walking` true)
  (set `self.Sitting` false)
  (set `self.Seated` false)
  (set `self.Still` false)
  (`KismetSystemLibrary.Delay` 4.0)
  (`KismetSystemLibrary.MoveComponentTo` (`self.Camera`) (-3000.0 0.0 1500.0) (struct) true true 5.0))

(event `CharaSitting`
  (set `self.Walking` false)
  (set `self.Sitting` true)
  (set `self.Seated` false)
  (set `self.Still` false))

(event `CharaSeated`
  (set `self.Walking` false)
  (set `self.Sitting` false)
  (set `self.Seated` true)
  (set `self.Still` false))

(event `ChangeFlameValue`
  (params (bIsChangeFlameValueActive :type Boolean))
  ;[0.4978 0.4978 0.4978] Smoke
  (if bIsChangeFlameValueActive
    (`ActorComponent.Activate` (`self.Smoke`) false)
    (else
      (`ActorComponent.Deactivate` (`self.Smoke`)))))

(event `CharaIdleSit`
  (set `self.Walking` false)
  (set `self.Sitting` false)
  (set `self.Seated` true)
  (set `self.Still` false))

(event `CharaIdleStand`
  (set `self.Still` true))

(event `WallGrabEvent` :!signature `self.WallGrabDelegate`
  (params (bIsGrabbing :type Boolean) (Offset :type "Float (single-precision)"))
  (bind (_relativelocation_x _relativelocation_y _relativelocation_z) (`KismetMathLibrary.BreakVector` (`SceneComponent.RelativeLocation` (`self.Sprite`))))
  (if bIsGrabbing
    (`SceneComponent.K2_SetRelativeLocation` (`self.Sprite`) (`KismetMathLibrary.MakeVector` (`KismetMathLibrary.SelectFloat` (+ Offset (`self.SpriteOffset`)) (- Offset (`self.SpriteOffset`)) (< Offset 0.0)) _relativelocation_y _relativelocation_z) false false)
    (else
      (`SceneComponent.K2_SetRelativeLocation` (`self.Sprite`) (`KismetMathLibrary.MakeVector` Offset _relativelocation_y _relativelocation_z) false false))))

(event `PlayerShoved`)

(event `DisableGravity`
  (bind _charactermovement (`self.CharacterMovement`))
  (bind _aspfecharacter_movement_component (cast `PFECharacterMovementComponent` _charactermovement))
  (set `PFECharacterMovementComponent.GlobalGravityScale` 0.0 _aspfecharacter_movement_component)
  (set `CharacterMovementComponent.GravityScale` 0.0 _charactermovement)
  (`PrimitiveComponent.SetEnableGravity` (`self.CapsuleComponent`) false))

(event `Key|A`
  (params (Key :type "Key Structure")))

(event `self.ReceiveTick`
  (params (DeltaSeconds :type "Float (single-precision)"))
  (bind _returnvalue_x (`KismetMathLibrary.BreakVector` (`SceneComponent.K2_GetComponentLocation` (`self.Camera`))))
  (`|ExecutionSequence`
    (:`then_0`
      ;[1 1 1] Reflexion
      (`self.SetReflexionPlaneRotation`)
      (`self.SetCameraReflexionRotation`)
      (for _array_element (`self.DynamicLayers`)
        (`MaterialInstanceDynamic.SetScalarParameterValue` _array_element "CameraPosX" _returnvalue_x)
        (`SceneComponent.K2_SetRelativeRotation` (`self.SpherePostProcess`) (select `bool` (< (`self.MoveValue`) 0.0) :`false` (`KismetMathLibrary.MakeRotator` 0.0 0.0 90.0) :`true` (`KismetMathLibrary.MakeRotator` 0.0 0.0 -90.0)) false false)))
    (:`then_1`
      (if (`|EnumInequality` (`FlameComponent.CurrentZoneEffect` (`self.Flame`)) "NORMAL")
        (`self.FlamePulse`)
        (else
          (`PaperFlipbookComponent.SetSpriteColor` (`self.Sprite`) (`self.ColorNormal`)))))
    (:`then_2`
      (bind _returnvalue (`GameplayStatics.GetCurrentLevelName` true))
      (if (not (`KismetStringLibrary.EqualEqual_StrStr` _returnvalue "TUNNEL_Level"))
        (`self.Set Camera XOffset` DeltaSeconds)))
    (:`then_3`
      (`PlayerController.SetAudioListenerOverride` :`self` (`GameplayStatics.GetPlayerController` 0) :`Location` (`self.K2_GetActorLocation`)))))

(fn `ChangeSpriteColor`
  (params (InColor :type "LinearColor Structure"))
  (`PaperFlipbookComponent.SetSpriteColor` (`self.Sprite`) InColor))

(fn `FlamePulse`
  (locals (DangerFactor :type "Float (double-precision)") (PulseValue :type "Float (double-precision)") (BaseColor :type "LinearColor Structure") (PulseColor :type "LinearColor Structure") (PulseSpeed :type "Float (double-precision)"))
  (bind _output_get (set `local.DangerFactor` (/ (`KismetMathLibrary.Abs` (- 50.0 (`FlameComponent.CurrentFlameValue` (`self.Flame`)))) 50.0)))
  (set `local.PulseSpeed` (`KismetMathLibrary.Lerp` 1.0 4.0 _output_get))
  (set `local.PulseValue` (/ (+ (`KismetMathLibrary.Sin` (* (`KismetSystemLibrary.GetGameTimeInSeconds`) (`local.PulseSpeed`))) 1.0) 2.0))
  (bind _output_get_2 (set `local.BaseColor` (select `EZoneEffect` (`FlameComponent.CurrentZoneEffect` (`self.Flame`)) :`DECREASE` (`self.ColorLow`) :`NORMAL` (`self.ColorNormal`) :`INCREASE` (`self.ColorHigh`))))
  (`PaperFlipbookComponent.SetSpriteColor` (`self.Sprite`) (`KismetMathLibrary.LinearColorLerp` (struct :`R` 1.0 :`G` 1.0 :`B` 1.0 :`A` 1.0) _output_get_2 (`KismetMathLibrary.FMin` 1.0 (* (* (`local.PulseValue`) (`KismetMathLibrary.Lerp` 0.5 1.0 (`local.DangerFactor`))) 1.2)))))

(fn `FlipCharacter`
  ;[1 0.9768 0.4373] Flip player
  (`Controller.SetControlRotation` (`self.GetController`) (select `bool` (< (`self.MoveValue`) 0.0) :`false` (`KismetMathLibrary.MakeRotator` 0.0) :`true` (`KismetMathLibrary.MakeRotator` 0.0 0.0 180.0))))

(fn `Set Camera XOffset`
  (params (DeltaTime :type "Float (double-precision)"))
  (bind _targetoffset_x (`KismetMathLibrary.BreakVector` (`SpringArmComponent.TargetOffset` (`self.SpringArm`))))
  (bind _targetoffset_x_2 (`KismetMathLibrary.BreakVector` (`SpringArmComponent.TargetOffset` (`self.SpringArm`))))
  (if (`self.GetIsLookingRight`)
    (set `SpringArmComponent.TargetOffset` (`KismetMathLibrary.MakeVector` (`KismetMathLibrary.FInterpTo` _targetoffset_x_2 200.0 DeltaTime 2.0)) (`self.SpringArm`))
    (else
      (set `SpringArmComponent.TargetOffset` (`KismetMathLibrary.MakeVector` (`KismetMathLibrary.FInterpTo` _targetoffset_x -200.0 DeltaTime 2.0)) (`self.SpringArm`)))))

(fn `SetCameraReflexionRotation`
  (bind _returnvalue (< (`self.MoveValue`) 0.0))
  (bind _returnvalue_2 (select `bool` _returnvalue :`false` (`KismetMathLibrary.MakeRotator` 0.0 0.0 90.0) :`true` (`KismetMathLibrary.MakeRotator` 0.0 0.0 -90.0)))
  (bind _returnvalue_3 (select `bool` _returnvalue :`false` (`KismetMathLibrary.MakeVector` 0.0 -250.0) :`true` (`KismetMathLibrary.MakeVector` 0.0 250.0)))
  (`SceneComponent.K2_SetRelativeTransform` (`self.SceneCapture_Horizontal`) (`KismetMathLibrary.MakeTransform` _returnvalue_3 _returnvalue_2) false false)
  (`SceneComponent.K2_SetRelativeTransform` (`self.SceneCapture_Vertical`) (`KismetMathLibrary.MakeTransform` _returnvalue_3 _returnvalue_2) false false))

(fn `SetReflexionPlaneRotation`
  (locals (XLeftLocation :type "Vector Structure" :default (0.0 0.0 0.0)))
  (`SceneComponent.K2_SetRelativeRotation` (`self.ReflexionHorizontal`) (select `bool` (< (`self.MoveValue`) 0.0) :`false` (`KismetMathLibrary.MakeRotator` 90.0 180.0) :`true` (`KismetMathLibrary.MakeRotator` 90.0 180.0 180.0)) false false)
  (`SceneComponent.K2_SetRelativeRotation` (`self.ReflexionVertical`) (select `bool` (< (`self.MoveValue`) 0.0) :`false` (`KismetMathLibrary.MakeRotator` 90.0) :`true` (`KismetMathLibrary.MakeRotator` 90.0 0.0 180.0)) false false))

(fn `UserConstructionScript`)