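; BP_CameraBounds is a trigger-based camera bounds actor that registers itself with the main camera while the player character is inside it.
; At BeginPlay it gets PFECamera from BP_MainCamera and adds itself immediately if IsPlayerInBounds is true.
; TriggerZone begin and end overlaps with a PFECharacter add or remove these bounds on PFECamera and print debug messages.
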(event `self.ReceiveBeginPlay`
  (bind _returnvalue (`GameplayStatics.GetActorOfClass` "/Game/Blueprints/Cameras/BP_MainCamera.BP_MainCamera_C"))
  (set `self.PFECamera` (`/Game/Blueprints/Cameras/BP_MainCamera.PFECamera` _returnvalue))
  (if (== (`self.IsPlayerInBounds`) true)
    (`PFECameraComponent.AddBounds` (`self.PFECamera`) self)))

(event `self.TriggerZone.OnComponentBeginOverlap`
  (params (OverlappedComponent :type "PrimitiveComponent Object Reference") (OtherActor :type "Actor Object Reference") (OtherComp :type "PrimitiveComponent Object Reference") (OtherBodyIndex :type Integer) (bFromSweep :type Boolean) (SweepResult :type "HitResult Structure (by ref)"))
  (cast `PFECharacter` OtherActor)
  (`PFECameraComponent.AddBounds` (`self.PFECamera`) self)
  (`KismetSystemLibrary.PrintString` "Enter Bounds"))

(event `self.TriggerZone.OnComponentEndOverlap`
  (params (OverlappedComponent :type "PrimitiveComponent Object Reference") (OtherActor :type "Actor Object Reference") (OtherComp :type "PrimitiveComponent Object Reference") (OtherBodyIndex :type Integer))
  (cast `PFECharacter` OtherActor)
  (`PFECameraComponent.RemoveBounds` (`self.PFECamera`) self)
  (`KismetSystemLibrary.PrintString` "Exit Bounds"))

(fn `UserConstructionScript`)