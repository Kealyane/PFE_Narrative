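; BP_MainCamera is the main camera Blueprint, which drives a custom PFECamera to position the view around the PFECharacter.
; On BeginPlay it finds the PFECharacter and passes it to PFECamera, or deactivates its own CameraComponent when UseDefaultCamera is set.
; Each Tick it delegates movement to PFECamera's UpdateCameraPosition unless the default camera is in use, and a getter exposes PFECamera.
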(event `self.ReceiveBeginPlay`
  (bind _returnvalue (`GameplayStatics.GetActorOfClass` "/Script/PFE_Narrative.PFECharacter"))
  (bind _output_get (set `self.PFECharacter` _returnvalue))
  (if (`PFECameraComponent.bUseDefaultCamera` (`self.PFECamera`))
    (`ActorComponent.Deactivate` (`self.CameraComponent`))
    (else
      (`/Engine/EditorBlueprintResources/StandardMacros.IsValid` _output_get
        (:`Is Valid`
          (`PFECameraComponent.SetPFECharacter` (`self.PFECamera`) (`self.PFECharacter`)))))))

(event `self.ReceiveTick`
  (params (DeltaSeconds :type "Float (single-precision)"))
  (if (not (`PFECameraComponent.bUseDefaultCamera` (`self.PFECamera`)))
    (`PFECameraComponent.UpdateCameraPosition` (`self.PFECamera`) DeltaSeconds)))

(fn `GetPFECamera`
  (returns (CameraComp :type "PFECameraComponent Object Reference"))
  (return (`self.PFECamera`)))

(fn `UserConstructionScript`)