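; BP_GameBounds is an out-of-bounds death volume that kills the player on overlap, as either liquid or ground.
; BeginPlay hides its render component and makes CollisionPlouf block pawns for liquid or in the tunnel level.
; Overlap freezes the player, flags drowning and plays a magma, water or ground sound chosen by SetSound.
; It then fades and reloads the level if HasDied is set without a checkpoint, otherwise launches the GameMode's death event.
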(event `self.ReceiveBeginPlay`
  (add `self.OnActorBeginOverlap` (delegate `OnActorBeginOverlap_Event`))
  (`SceneComponent.SetVisibility` (`self.RenderComponent`) false false)
  (bind _returnvalue (`GameplayStatics.GetCurrentLevelName` true))
  (if (or (`self.bIsLiquid`) (== _returnvalue "TUNNEL_Level"))
    (`PrimitiveComponent.SetCollisionResponseToChannel` (`self.CollisionPlouf`) "ECC_Pawn" "ECR_Block")
    (else
      (`PrimitiveComponent.SetCollisionResponseToChannel` (`self.CollisionPlouf`) "ECC_Pawn" "ECR_Ignore"))))

(event `OnActorBeginOverlap_Event` :!signature `self.OnActorBeginOverlap`
  (params (OverlappedActor :type "Actor Object Reference") (OtherActor :type "Actor Object Reference"))
  (bind _asbp_player (cast `/Game/Characters/Player/Blueprints/BP_Player` OtherActor))
  (set `PFECharacter.bCanMove` false _asbp_player)
  (set `/Game/Characters/Player/Blueprints/BP_Player.IsDrowning` true _asbp_player)
  (`self.SetSound`)
  (`AudioComponent.Play` (`self.Audio`) 0.0)
  ;[0.5135 0.9325 1] Reload Level if has not reach a checkpoint
  (bind _asbp_pfegame_instance (cast `/Game/Blueprints/Core/BP_PFEGameInstance` (`GameplayStatics.GetGameInstance`)))
  (if (and (`PFEGameInstance.bHasDied` _asbp_pfegame_instance) (not (`PFEGameInstance.bHasReachCheckpoint` _asbp_pfegame_instance)))
    (`KismetSystemLibrary.PrintString` "BP_GameBounds::Reload level has died ans has not reach checkpoint" true true (struct :`G` 0.66 :`B` 1.0 :`A` 1.0) 5.0)
    (bind _foundwidgets (`WidgetBlueprintLibrary.GetAllWidgetsOfClass` "/Game/UI/Widgets/HUD/WBP_FadeScreen.WBP_FadeScreen_C"))
    (`/Game/UI/Widgets/HUD/WBP_FadeScreen.ScreenFadeIn` (`|GetArrayItem` _foundwidgets))
    (`KismetSystemLibrary.Delay` 1.0)
    (`/Game/Blueprints/Core/BP_PFEGameInstance.Mute` _asbp_pfegame_instance)
    (bind _levelpath (`/Game/Blueprints/Core/BP_PFEGameInstance.GetLevelPath` _asbp_pfegame_instance (`/Game/Blueprints/Core/BP_PFEGameInstance.CurrentLevel` _asbp_pfegame_instance)))
    (`GameplayStatics.OpenLevel` (`KismetStringLibrary.Conv_StringToName` _levelpath))
    (else
      (bind _aspfegame_mode (cast `PFEGameMode` (`GameplayStatics.GetGameMode`)))
      (`PFEGameMode.LaunchDeathEvent` _aspfegame_mode)
      (`KismetSystemLibrary.Delay` 1.0)
      (set `/Game/Characters/Player/Blueprints/BP_Player.IsDrowning` false _asbp_player))))

(fn `SetSound`
  (if (`self.bIsLiquid`)
    (bind _returnvalue (`GameplayStatics.GetCurrentLevelName` true))
    (if (== _returnvalue "BURN_OUT_Level")
      (`AudioComponent.SetSound` (`self.Audio`) (`self.MagmaSound`))
      (else
        (`AudioComponent.SetSound` (`self.Audio`) (`self.WaterSound`))))
    (else
      (`AudioComponent.SetSound` (`self.Audio`) (`self.GroundSound`)))))

(fn `UserConstructionScript`)