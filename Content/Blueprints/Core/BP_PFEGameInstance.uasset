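; PFE game instance that holds the current level and save, and provides level lookup and master audio muting.
; Data tables translate between level enums and paths, with substring matching for the reverse lookup.
; The save loads from a slot to restore the current level, while SaveLevel only updates that object in memory.
; Mute and Unmute override the master sound class volume through a sound mix.
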(fn `GetEnumFromPath`
  (params (LevelName :type String))
  (returns (Level :type "/Game/Datas/ELevelsName Enum"))
  (bind _outrownames (`DataTableFunctionLibrary.GetDataTableRowNames` (`self.DT_Level`)))
  (for _array_element _outrownames
    (bind _returnvalue (`|GetDataTableRow` "/Game/Datas/DT_LevelsPath.DT_LevelsPath" _array_element)
      (:`then`
        (if (`KismetStringLibrary.Contains` (`.Path_5_B8595AA94BD2A9EF93216B87BF4D8BE2` (break `/Game/Datas/S_LevelPath` _returnvalue)) LevelName)
          (return (break `/Game/Datas/S_LevelPath` _returnvalue))))))
  (`KismetSystemLibrary.PrintString` "BP_GameInstance::GetEnumFromPath no matching level name and path" true true (struct :`R` 1.0 :`G` 0.016636 :`A` 1.0) 10.0)
  (return "NewEnumerator0"))

(fn `GetLevelPath`
  (params (Level :type "/Game/Datas/ELevelsName Enum" :default "NewEnumerator0"))
  (returns (LevelPath :type String))
  (bind _returnvalue (`|GetDataTableRow` (`self.DT_Level`) (`KismetStringLibrary.Conv_StringToName` (`|GetEnumeratorNameAsString` Level)))
    (:`then`
      (return (`.Path_5_B8595AA94BD2A9EF93216B87BF4D8BE2` (break `/Game/Datas/S_LevelPath` _returnvalue))))))

(fn `LoadLevelFromSave`
  (bind _currentsave (`self.CurrentSave`))
  (`/Engine/EditorBlueprintResources/StandardMacros.IsValid` _currentsave
    (:`Is Valid`
      _)
    (:`Is Not Valid`
      (`self.SetCurrentSave`)))
  (set `self.CurrentLevel` (cast `/Game/Datas/ELevelsName` (`PFESaveGame.LevelToLoad` _currentsave))))

(fn `Mute`
  (`GameplayStatics.SetSoundMixClassOverride` "/Game/Sounds/Mixer/MasterSoundMix.MasterSoundMix" "/Game/Sounds/Mixer/SC_Master.SC_Master" 0.0 1.0 0.0))

(fn `SaveLevel`
  (params (LevelToSave :type Byte))
  (bind _currentsave (`self.CurrentSave`))
  (`/Engine/EditorBlueprintResources/StandardMacros.IsValid` _currentsave
    (:`Is Valid`
      (set `PFESaveGame.LevelToLoad` LevelToSave _currentsave))))

(fn `SetCurrentSave`
  (bind _returnvalue (`GameplayStatics.LoadGameFromSlot` (`self.SlotName`)))
  (bind _aspfesave_game (cast `PFESaveGame` _returnvalue))
  (set `self.CurrentSave` _aspfesave_game))

(fn `Unmute`
  (`GameplayStatics.SetSoundMixClassOverride` "/Game/Sounds/Mixer/MasterSoundMix.MasterSoundMix" "/Game/Sounds/Mixer/SC_Master.SC_Master" (`self.SoundLevelMaster`)))