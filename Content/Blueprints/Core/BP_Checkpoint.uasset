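; BP_Checkpoint is a checkpoint actor that shows its active state with an animated Paper2D flipbook and a sound.
; On BeginPlay it hides the flipbook and initializes its Sound component.
; The UpdateCheckpoint event takes an active flag: when true it shows and loops the flipbook and plays the Checkpoint sound, otherwise it stops and hides the flipbook.
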(event `self.ReceiveBeginPlay`
  (`SceneComponent.SetVisibility` (`self.PaperFlipbook`) false false)
  (`self.InitSoundComponent` (`self.Sound`)))

(event `self.UpdateCheckpoint`
  (params (InIsActive :type Boolean))
  (bind _paperflipbook (`self.PaperFlipbook`))
  (if InIsActive
    (`SceneComponent.SetVisibility` _paperflipbook true false)
    (`PaperFlipbookComponent.SetLooping` _paperflipbook true)
    (`PaperFlipbookComponent.Play` _paperflipbook)
    (`SoundComponent.PlaySound` (`self.Sound`) "Checkpoint")
    (else
      (`PaperFlipbookComponent.Stop` (`self.PaperFlipbook`))
      (`SceneComponent.SetVisibility` (`self.PaperFlipbook`) false false))))

(fn `UserConstructionScript`)