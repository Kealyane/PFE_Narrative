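; BP_Door is a 2D sprite door that opens when an open-door delegate fires, serving as either a regular door or a trapdoor.
; It binds to the delegate on BeginPlay, then plays a sound, swaps the sprite according to IsNotTrapdoor, and disables collision on the box and door.
; An unused flipbook animation branch remains in the graph but never runs.
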(event `self.ReceiveBeginPlay`
  (add `self.OpenDoorDelegate` (delegate `OnOpenDoor`)))

(event `OnOpenDoor`
  (`GameplayStatics.PlaySound2D` "/Game/Sounds/DoorSound_Cue.DoorSound_Cue" 1.0 1.0 0.0 null null)
  (if (`self.IsNotTrapdoor`)
    (`PaperSpriteComponent.SetSprite` (`self.Door`) "/Game/Sprites/Door/Portes_Key-2_Sprite_0.Portes_Key-2_Sprite_0")
    (else
      (`PaperSpriteComponent.SetSprite` (`self.Door`) "/Game/Sprites/Door/trapdoor_open_Sprite_0.trapdoor_open_Sprite_0")))
  (`PrimitiveComponent.SetCollisionEnabled` (`self.Box`) "NoCollision")
  (`PrimitiveComponent.SetCollisionEnabled` (`self.Door`) "NoCollision"))

(fn `UserConstructionScript`)