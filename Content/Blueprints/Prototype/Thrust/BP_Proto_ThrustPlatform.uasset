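; Prototype thrust platform that carries the player horizontally while their flame status controls vertical movement.
; On first overlap with a PFECharacter, it closes the left pawn blocker after a short delay and starts moving via AllowMove.
; Small flame sinks, normal stays level and high rises, with Z speed updated through the player's flame-status delegate.
; When the platform stops, the bound stop event opens the right blocker to pawns.
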(event `self.ReceiveBeginPlay`
  (`PrimitiveComponent.SetCollisionResponseToChannel` (`self.BlockerLeft`) "ECC_Pawn" "ECR_Ignore")
  (add `self.OnStopPlatform` (`|CreateDelegate` :!event `OnStop`)))

(event `self.Overlap.OnComponentBeginOverlap`
  (params (OverlappedComponent :type "PrimitiveComponent Object Reference") (OtherActor :type "Actor Object Reference") (OtherComp :type "PrimitiveComponent Object Reference") (OtherBodyIndex :type Integer) (bFromSweep :type Boolean) (SweepResult :type "HitResult Structure (by ref)"))
  (bind _aspfecharacter (cast `PFECharacter` OtherActor))
  (set `self.Player` _aspfecharacter)
  (if (not (`self.OverlapDone`))
    (set `self.OverlapDone` true)
    (add `PFECharacter.FlameStatusChangedDelegate` (`self.Player`) (`|CreateDelegate` :!event `OnFlameStatusChanged`))
    (`KismetSystemLibrary.Delay` 0.8)
    (`PrimitiveComponent.SetCollisionResponseToChannel` (`self.BlockerLeft`) "ECC_Pawn" "ECR_Block")
    ;[0.4645 0.6986 0.4136] Active Tick and Set Movement Speed
    (`self.AllowMove` 300.0 (select `EFlameStatus` (`PFECharacter.GetFlameStatus` (`self.Player`)) :`SMALL` -200.0 :`HIGH` 200.0))))

(event `OnFlameStatusChanged`
  (params (FlameStatus :type "EFlameStatus Enum" :default "SMALL"))
  ;[0.317 0.555 0.3034] When Flame Changed -> Modify Z Speed Here
  (`self.SetZSpeed` (select `EFlameStatus` FlameStatus :`SMALL` -200.0 :`HIGH` 200.0)))

(event `OnStop`
  (`PrimitiveComponent.SetCollisionResponseToChannel` (`self.BlockerRight`) "ECC_Pawn" "ECR_Ignore")
  (`KismetSystemLibrary.PrintString` "ThrustPlatform : Stop" true true (struct :`R` 1.0 :`G` 0.270895 :`B` 0.253068 :`A` 1.0) 5.0))

(fn `UserConstructionScript`)