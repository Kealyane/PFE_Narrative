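; BP_Lift is a lift that carries itself to a Destination actor's location and back after BP_Player enters its collider.
; A DoOnce starts the TimerUp timeline as a countdown, which any actor end overlap stops.
; When the timeline finishes, a sound plays and eased MoveComponentTo calls move the root out, pause briefly, then return it to its BeginPlay location.
; The DoOnce resets only after the return trip.
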(event `self.ReceiveBeginPlay`
  (bind _returnvalue (`GameplayStatics.GetActorOfClass` "/Game/Blueprints/Player/BP_Player.BP_Player_C"))
  (set `self.PlayerRef` _returnvalue)
  (set `self.DefaultLoc` (`SceneComponent.K2_GetComponentLocation` (`self.DefaultSceneRoot`))))

(event `self.Collider.OnComponentBeginOverlap`
  (params (OverlappedComponent :type "PrimitiveComponent Object Reference") (OtherActor :type "Actor Object Reference") (OtherComp :type "PrimitiveComponent Object Reference") (OtherBodyIndex :type Integer) (bFromSweep :type Boolean) (SweepResult :type "HitResult Structure (by ref)"))
  (bind (_returnvalue_x _returnvalue_y _returnvalue_z) (`KismetMathLibrary.BreakVector` (`SceneComponent.K2_GetComponentLocation` (`/Game/Blueprints/TMP/BP_LiftDestination.DefaultSceneRoot` (`self.Destination`)))))
  (cast `/Game/Blueprints/Player/BP_Player` OtherActor)
  (`/Engine/EditorBlueprintResources/StandardMacros.DoOnce` false :!label _label
    (:`Completed`
      (`Timeline|TimerUp` :!via `PlayFromStart` :!label _label_2
        (:`Finished`
          (`|ExecutionSequence`
            (:`then_0`
              (`GameplayStatics.PlaySound2D` "/Game/Sounds/Lift_Cue.Lift_Cue" 1.0 1.0 0.0 null null))
            (:`then_1`
              _))
          (`KismetSystemLibrary.MoveComponentTo` (`self.DefaultSceneRoot`) (`KismetMathLibrary.MakeVector` _returnvalue_x _returnvalue_y _returnvalue_z) (struct) true true (`self.TimeToReach`))
          (`KismetSystemLibrary.Delay` 1.0)
          (`KismetSystemLibrary.MoveComponentTo` (`self.DefaultSceneRoot`) (`self.DefaultLoc`) (struct) true true (`self.TimeToReach`))
          (`self.ResetDoOnce`))))))

(event `ResetDoOnce`
  (goto _label :!via `Reset`))

(event `Stop`
  (goto _label_2 :!via `Stop`))

(event `self.ReceiveActorEndOverlap`
  (params (OtherActor :type "Actor Object Reference"))
  (`self.Stop`))

(fn `UserConstructionScript`)