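; Crumbling 2D platform that breaks after the player touches it and later reforms.
; Trigger overlap launches inherited destroy timers, whose state-change callback swaps Paper2D flipbooks, visibility and Pawn collision responses.
; While broken, the Collider switches from Block to Overlap to detect a player inside, deferring restoration until they leave.
; A timed restore restarts the destroy timers if the player is still in the Trigger.
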(event `self.ReceiveBeginPlay`
  (add `self.StateChanged` (delegate `OnStateChanged`))
  (`self.InitSoundComponent` (`self.Sound`))
  (`self.PlatformVisibleCollisions`))

(event `OnStateChanged` :!signature `self.StateChanged`
  (params (bIsPlatformDestroyed :type Boolean))
  (bind _fb_platformbreak1 (`self.FB_PlatformBreak1`))
  ;[1 1 1] event platform destroyed
  (if bIsPlatformDestroyed
    ;[1 0.3867 0.3824] platform destroyed (player can't step on it)
    (`self.PlatformDestroyedCollisions`)
    (`PaperFlipbookComponent.SetFlipbook` _fb_platformbreak1 "/Game/Interactables/Platforms/Break/Flipbooks/FB_PlatformBreak.FB_PlatformBreak")
    (`KismetSystemLibrary.Delay` 0.5)
    (`SceneComponent.SetVisibility` _fb_platformbreak1 false false)
    (set `self.PlatformDestroyed` true)
    (set `self.CheckPlayer` true)
    (elif (not (`self.PlayerIn`))
      (`SceneComponent.SetVisibility` (`self.FB_PlatformBreak1`) true false)
      ;[0.5241 1 0.5806] platform intact (player can step on it)
      (`PaperFlipbookComponent.SetFlipbook` (`self.FB_PlatformBreak1`) "/Game/Interactables/Platforms/Break/Flipbooks/FB_PlatformBreakReverse.FB_PlatformBreakReverse")
      (`self.PlatformVisibleCollisions`)
      (set `self.PlatformDestroyed` false)
      (set `self.CheckPlayer` false)
      (`KismetSystemLibrary.Delay` 0.8)
      (`PaperFlipbookComponent.SetFlipbook` (`self.FB_PlatformBreak1`) "/Game/Interactables/Platforms/Break/Flipbooks/FB_PlatformBreak1.FB_PlatformBreak1")
      (if (`self.PlayerInTrigger`)
        (`self.LaunchTimersToDestroyPlatform`)))))

(event `self.Trigger.OnComponentBeginOverlap`
  (params (OverlappedComponent :type "PrimitiveComponent Object Reference") (OtherActor :type "Actor Object Reference") (OtherComp :type "PrimitiveComponent Object Reference") (OtherBodyIndex :type Integer) (bFromSweep :type Boolean) (SweepResult :type "HitResult Structure (by ref)"))
  (cast `PFECharacter` OtherActor)
  (`self.LaunchTimersToDestroyPlatform`)
  (set `self.PlayerInTrigger` true))

(event `self.Trigger.OnComponentEndOverlap`
  (params (OverlappedComponent :type "PrimitiveComponent Object Reference") (OtherActor :type "Actor Object Reference") (OtherComp :type "PrimitiveComponent Object Reference") (OtherBodyIndex :type Integer))
  (cast `PFECharacter` OtherActor)
  (set `self.PlayerInTrigger` false))

(event `self.Collider.OnComponentBeginOverlap`
  (params (OverlappedComponent :type "PrimitiveComponent Object Reference") (OtherActor :type "Actor Object Reference") (OtherComp :type "PrimitiveComponent Object Reference") (OtherBodyIndex :type Integer) (bFromSweep :type Boolean) (SweepResult :type "HitResult Structure (by ref)"))
  ;[0.4144 0.4144 0.4144] Check if player is in destroyed platform
  (cast `PFECharacter` OtherActor)
  (if (`self.CheckPlayer`)
    (set `self.PlayerIn` true)))

(event `self.Collider.OnComponentEndOverlap`
  (params (OverlappedComponent :type "PrimitiveComponent Object Reference") (OtherActor :type "Actor Object Reference") (OtherComp :type "PrimitiveComponent Object Reference") (OtherBodyIndex :type Integer))
  ;[0.4144 0.4144 0.4144] Check if player is in destroyed platform
  (cast `PFECharacter` OtherActor)
  (if (and (`self.PlayerIn`) (`self.PlatformDestroyed`) (`self.CheckPlayer`))
    (`SceneComponent.SetVisibility` (`self.FB_PlatformBreak1`) true false)
    ;;[0.5241 1 0.5806] platform intact (player can step on it)
    (`PaperFlipbookComponent.SetFlipbook` (`self.FB_PlatformBreak1`) "/Game/Interactables/Platforms/Break/Flipbooks/FB_PlatformBreakReverse.FB_PlatformBreakReverse")
    (`self.PlatformVisibleCollisions`)
    (set `self.PlayerIn` false)
    (set `self.PlatformDestroyed` false)
    (set `self.CheckPlayer` false)
    (`KismetSystemLibrary.Delay` 0.8)
    (`PaperFlipbookComponent.SetFlipbook` (`self.FB_PlatformBreak1`) "/Game/Interactables/Platforms/Break/Flipbooks/FB_PlatformBreak1.FB_PlatformBreak1")))

(fn `PlatformDestroyedCollisions`
  (`PrimitiveComponent.SetCollisionResponseToChannel` (`self.Collider`) "ECC_Pawn" "ECR_Overlap")
  (`PrimitiveComponent.SetCollisionResponseToChannel` (`self.Trigger`) "ECC_Pawn" "ECR_Ignore"))

(fn `PlatformVisibleCollisions`
  (`PrimitiveComponent.SetCollisionResponseToChannel` (`self.Collider`) "ECC_Pawn" "ECR_Block")
  (`PrimitiveComponent.SetCollisionResponseToChannel` (`self.Trigger`) "ECC_Pawn" "ECR_Overlap"))

(fn `UserConstructionScript`)