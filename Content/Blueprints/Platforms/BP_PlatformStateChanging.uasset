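; Platform actor that shows its open or closed state by tinting its sprite.
; On BeginPlay it binds to a status-changed event and sets the initial color from the AtStartIsOpen flag.
; Each status change then switches the RenderComponent sprite between the Open and Close colors.
; The graph handles only this visual feedback, with no overlap, tick or construction logic.
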(event `self.ReceiveBeginPlay`
  (bind _rendercomponent (`self.RenderComponent`))
  (add `self.StatusChanged` (delegate `OnStatusChanged`))
  (if (`self.bAtStartIsOpen`)
    (`PaperSpriteComponent.SetSpriteColor` _rendercomponent (`self.Open`))
    (else
      (`PaperSpriteComponent.SetSpriteColor` _rendercomponent (`self.Close`)))))

(event `OnStatusChanged` :!signature `self.StatusChanged`
  (params (bIsPlatformOpen :type Boolean))
  (bind _rendercomponent (`self.RenderComponent`))
  (if bIsPlatformOpen
    (`PaperSpriteComponent.SetSpriteColor` _rendercomponent (`self.Open`))
    (else
      (`PaperSpriteComponent.SetSpriteColor` _rendercomponent (`self.Close`)))))

(fn `UserConstructionScript`)