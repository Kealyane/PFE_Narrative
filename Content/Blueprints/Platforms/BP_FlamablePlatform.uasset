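; Flamable platform that burns away, hiding its sprite and ignoring collision, when a BP_Player with a high enough flame value enters its trigger.
; If it has connected platforms, it then hides and disables them one by one through a latent DelayedLoop macro spaced by a shared delay.
; When the chain finishes, or immediately if there is none, it lights the brazier of its connected torch, if one is set.
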(event `self.ReceiveBeginPlay`
  (`|ExecutionSequence`
    (:`then_0`
      (if (!= (`KismetArrayLibrary.Array_Length` (`self.ConnectedPlatforms`)) 0)
        (set `self.IsConnectedToOther` true)
        (else
          (`KismetArrayLibrary.Array_Clear` (`self.ConnectedPlatforms`)))))
    (:`then_1`
      (`/Engine/EditorBlueprintResources/StandardMacros.IsValid` (`self.ConnectedTorch`)
        (:`Is Valid`
          (set `self.IsTorchConnected` true))
        (:`Is Not Valid`
          (set `self.IsTorchConnected` false))))))

(event `self.ReceiveActorBeginOverlap`
  (params (OtherActor :type "Actor Object Reference")))

(event `self.Trigger.OnComponentBeginOverlap`
  (params (OverlappedComponent :type "PrimitiveComponent Object Reference") (OtherActor :type "Actor Object Reference") (OtherComp :type "PrimitiveComponent Object Reference") (OtherBodyIndex :type Integer) (bFromSweep :type Boolean) (SweepResult :type "HitResult Structure (by ref)"))
  (bind _asbp_player (cast `/Game/Blueprints/Player/BP_Player` OtherActor))
  (if (>= (`FlameComponent.GetFlameValue` (`/Game/Blueprints/Player/BP_Player.Flame` _asbp_player)) 70.0)
    (`SceneComponent.SetVisibility` (`self.PaperSprite`) false false)
    (`PrimitiveComponent.SetCollisionResponseToAllChannels` (`self.Collision`) "ECR_Ignore")
    (if (`self.IsConnectedToOther`)
      (`KismetSystemLibrary.Delay` (`self.DelayBetweenDetruct`))
      (bind _arrayelement (`self.DelayedLoop` (`self.DelayBetweenDetruct`) (`self.ConnectedPlatforms`))
        (:`Loop`
          (`SceneComponent.SetVisibility` (`/Game/Blueprints/Platforms/BP_FlamablePlatform.PaperSprite` _arrayelement) false false)
          (`PrimitiveComponent.SetCollisionResponseToAllChannels` (`/Game/Blueprints/Platforms/BP_FlamablePlatform.Collision` _arrayelement) "ECR_Ignore"))
        (:`Completed`
          (if (`self.IsTorchConnected`) :!label _label
            (`/Game/Blueprints/Level/Doors/BP_FlameForDoor.LightBrasero` (`self.ConnectedTorch`)))))
      (else
        (goto _label)))))

(fn `UserConstructionScript`)