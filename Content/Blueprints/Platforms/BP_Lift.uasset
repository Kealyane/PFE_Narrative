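; BP_Lift is a platform that moves to a Destination actor's location after the player steps into its Collider.
; The overlap restarts the TimerUp timeline as a delay, and its finish triggers an eased MoveComponentTo on the root over TimeToReach.
; Any actor overlap ending stops the timeline, cancelling a pending departure.
; The start location and player reference are cached at BeginPlay but unused, and no return movement exists.
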(event `self.ReceiveBeginPlay`
  (bind _returnvalue (`GameplayStatics.GetActorOfClass` "/Game/Blueprints/Player/BP_Player.BP_Player_C"))
  (set `self.PlayerRef` _returnvalue)
  (set `self.DefaultLoc` (`SceneComponent.K2_GetComponentLocation` (`self.DefaultSceneRoot`))))

(event `self.Collider.OnComponentBeginOverlap`
  (params (OverlappedComponent :type "PrimitiveComponent Object Reference") (OtherActor :type "Actor Object Reference") (OtherComp :type "PrimitiveComponent Object Reference") (OtherBodyIndex :type Integer) (bFromSweep :type Boolean) (SweepResult :type "HitResult Structure (by ref)"))
  (bind (_returnvalue_x _returnvalue_y _returnvalue_z) (`KismetMathLibrary.BreakVector` (`SceneComponent.K2_GetComponentLocation` (`/Game/Blueprints/Platforms/BP_LiftDestination.DefaultSceneRoot` (`self.Destination`)))))
  (cast `/Game/Blueprints/Player/BP_Player` OtherActor)
  (`Timeline|TimerUp` :!via `PlayFromStart` :!label _label
    (:`Finished`
      (`KismetSystemLibrary.MoveComponentTo` (`self.DefaultSceneRoot`) (`KismetMathLibrary.MakeVector` _returnvalue_x _returnvalue_y _returnvalue_z) (struct) true true (`self.TimeToReach`)))))

(event `Stop`
  (goto _label :!via `Stop`))

(event `self.ReceiveActorEndOverlap`
  (params (OtherActor :type "Actor Object Reference"))
  (`self.Stop`))

(fn `UserConstructionScript`)