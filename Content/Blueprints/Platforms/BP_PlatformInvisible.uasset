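; Invisible platform that shows a mirror-platform Niagara effect while the player stands on it.
; When BP_Player begins overlapping, it stores the render component's location, spawns NS_MirrorPlatform there and starts a looping timer.
; The timer respawns the effect every two seconds while the on-platform flag is set.
; Any end overlap clears the flag and timer, without checking which actor left.
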(event `self.ReceiveBeginPlay`
  (bind _returnvalue (`GameplayStatics.GetActorOfClass` "/Game/Blueprints/Player/BP_Player.BP_Player_C"))
  (set `self.PlayerRef` _returnvalue))

(event `self.ReceiveActorBeginOverlap`
  (params (OtherActor :type "Actor Object Reference"))
  (bind (_returnvalue_x _returnvalue_y _returnvalue_z) (`KismetMathLibrary.BreakVector` (`SceneComponent.K2_GetComponentLocation` (`self.RenderComponent`))))
  (cast `/Game/Blueprints/Player/BP_Player` OtherActor)
  (set `self.StillOnPlarform` true)
  (bind _output_get (set `self.PlatformLoc` (`KismetMathLibrary.MakeVector` _returnvalue_x _returnvalue_y _returnvalue_z)))
  (`NiagaraFunctionLibrary.SpawnSystemAtLocation` "/Game/VFX/NS_MirrorPlatform.NS_MirrorPlatform" (`KismetMathLibrary.MakeVector` (.x _output_get) (.y _output_get) (.z _output_get)))
  (bind _returnvalue (`KismetSystemLibrary.K2_SetTimerDelegate` (delegate `CheckPlayerStillOnPlat`) 2.0 true))
  (set `self.Timer` _returnvalue))

(event `CheckPlayerStillOnPlat`
  (if (`self.StillOnPlarform`)
    (`NiagaraFunctionLibrary.SpawnSystemAtLocation` "/Game/VFX/NS_MirrorPlatform.NS_MirrorPlatform" (`self.PlatformLoc`))))

(event `self.ReceiveActorEndOverlap`
  (params (OtherActor :type "Actor Object Reference"))
  (set `self.StillOnPlarform` false)
  (`KismetSystemLibrary.K2_ClearAndInvalidateTimerHandle` (`self.Timer`)))

(fn `UserConstructionScript`)