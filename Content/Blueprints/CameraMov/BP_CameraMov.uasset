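; BP_CameraMov is a trigger volume that shifts the player's camera while BP_Player is inside its Box.
; On overlap begin, a Timeline drives a Lerp of the camera's relative location from the player's CameraInitPos to CameraMovesTo.
; On overlap end, the same Timeline reverses, easing the camera back.
; BeginPlay caches a PlayerRef, but the movement uses the overlapping actor's cast instead.
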(event `self.ReceiveBeginPlay`
  (bind _returnvalue (`GameplayStatics.GetActorOfClass` "/Game/Blueprints/Player/BP_Player.BP_Player_C"))
  (set `self.PlayerRef` _returnvalue))

(event `self.Box.OnComponentBeginOverlap`
  (params (OverlappedComponent :type "PrimitiveComponent Object Reference") (OtherActor :type "Actor Object Reference") (OtherComp :type "PrimitiveComponent Object Reference") (OtherBodyIndex :type Integer) (bFromSweep :type Boolean) (SweepResult :type "HitResult Structure (by ref)"))
  (bind _asbp_player (cast `/Game/Blueprints/Player/BP_Player` OtherActor))
  (bind (_direction _newtrack_0) (`Timeline|Timeline` :!label _label)
    (:`Update`
      (`SceneComponent.K2_SetRelativeLocation` (`PFECharacter.Camera` _asbp_player) (`KismetMathLibrary.VLerp` (`/Game/Blueprints/Player/BP_Player.CameraInitPos` _asbp_player) (`self.CameraMovesTo`) _newtrack_0) false false))))

(event `self.Box.OnComponentEndOverlap`
  (params (OverlappedComponent :type "PrimitiveComponent Object Reference") (OtherActor :type "Actor Object Reference") (OtherComp :type "PrimitiveComponent Object Reference") (OtherBodyIndex :type Integer))
  (cast `/Game/Blueprints/Player/BP_Player` OtherActor)
  (goto _label :!via `Reverse`))

(fn `UserConstructionScript`)