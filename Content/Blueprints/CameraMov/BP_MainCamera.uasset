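; Main camera actor that wraps a PFECamera and links it to the PFECharacter in the level.
; On BeginPlay it finds the character and, in default-camera mode, snaps itself once to the character's X and Z at the camera's configured Y.
; Otherwise it hands a valid character to the PFECamera and prints whether that succeeded.
; Tick is unused, and a getter exposes the PFECamera.
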(event `self.ReceiveBeginPlay`
  (bind (_returnvalue_x _returnvalue_y _returnvalue_z) (`KismetMathLibrary.BreakVector` (`self.K2_GetActorLocation` (`self.PFECharacter`))))
  (bind _returnvalue (`GameplayStatics.GetActorOfClass` "/Script/PFE_Narrative.PFECharacter"))
  (bind _output_get (set `self.PFECharacter` _returnvalue))
  (if (`PFECameraComponent.bUseDefaultCamera` (`self.PFECamera`))
    (bind _output_get_2 (set `self.CameraInitPos` (`KismetMathLibrary.MakeVector` _returnvalue_x (`PFECameraComponent.YLocation` (`self.PFECamera`)) _returnvalue_z)))
    (`self.K2_SetActorLocation` _output_get_2)
    (else
      (`/Engine/EditorBlueprintResources/StandardMacros.IsValid` _output_get
        (:`Is Valid`
          (`PFECameraComponent.SetPFECharacter` (`self.PFECamera`) (`self.PFECharacter`))
          (`KismetSystemLibrary.PrintString` "main camera : set pfe chara" true true (struct :`R` 0.18218 :`G` 1.0 :`A` 1.0)))
        (:`Is Not Valid`
          (`KismetSystemLibrary.PrintString` "main camera : fail set pfe chara" true true (struct :`R` 1.0 :`B` 0.098781 :`A` 1.0)))))))

(fn `GetPFECamera`
  (returns (CameraComp :type "PFECameraComponent Object Reference"))
  (return (`self.PFECamera`)))

(fn `UserConstructionScript`)