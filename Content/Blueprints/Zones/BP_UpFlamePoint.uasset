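; BP_UpFlamePoint is a reusable pickup zone that raises the player's flame life to a higher tier on overlap.
; ChangePlayerState checks which range PlayerLife falls in, sets it to the corresponding higher value, then calls CheckPlayerLife on the player reference cached at BeginPlay.
; A DoOnce gate limits triggering while the cube disables collision and swaps material, until the TimBeforeEnable timeline finishes and re-arms it.
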(event `self.ReceiveBeginPlay`
  (bind _returnvalue (`GameplayStatics.GetActorOfClass` "/Game/Blueprints/Player/BP_Player.BP_Player_C"))
  (set `self.PlayerRef` _returnvalue))

(event `self.ReceiveActorBeginOverlap`
  (params (OtherActor :type "Actor Object Reference"))
  (bind _cube (`self.Cube`))
  (bind _cube_2 (`self.Cube`))
  (`/Engine/EditorBlueprintResources/StandardMacros.DoOnce` false :!label _label
    (:`Completed`
      (cast `/Game/Blueprints/Player/BP_Player` OtherActor)
      (`self.ChangePlayerState`)
      (`PrimitiveComponent.SetCollisionEnabled` _cube_2 "NoCollision")
      (`PrimitiveComponent.SetMaterial` _cube_2 0 "/Game/Materials/M_DisabledPoint.M_DisabledPoint")
      (`Timeline|TimBeforeEnable` :!via `PlayFromStart`
        (:`Finished`
          (`PrimitiveComponent.SetCollisionEnabled` _cube "QueryOnly")
          (`PrimitiveComponent.SetMaterial` _cube 0 "/Game/Materials/M_Point+.M_Point+")
          (`self.ResetDoOnce`))))))

(event `ResetDoOnce`
  (goto _label :!via `Reset`))

(event `ChangePlayerState`
  (bind _playerref (`self.PlayerRef`))
  (bind _playerref_2 (`self.PlayerRef`))
  (bind _playerref_3 (`self.PlayerRef`))
  (bind _playerlife (`/Game/Blueprints/Player/BP_Player.PlayerLife` (`self.PlayerRef`)))
  (if (`KismetMathLibrary.InRange_IntInt` _playerlife 0 30 false)
    (set `/Game/Blueprints/Player/BP_Player.PlayerLife` (`self.DefaultFlameHP`) _playerref_3)
    (`/Game/Blueprints/Player/BP_Player.CheckPlayerLife` _playerref_3)
    (elif (`KismetMathLibrary.InRange_IntInt` _playerlife 30 70 false)
      (set `/Game/Blueprints/Player/BP_Player.PlayerLife` (`self.BigFlameHP`) _playerref_2)
      (`/Game/Blueprints/Player/BP_Player.CheckPlayerLife` _playerref_2)
      (elif (`KismetMathLibrary.InRange_IntInt` _playerlife 70 100 false)
        (set `/Game/Blueprints/Player/BP_Player.PlayerLife` 150 _playerref)
        (`/Game/Blueprints/Player/BP_Player.CheckPlayerLife` _playerref)))))

(fn `UserConstructionScript`)