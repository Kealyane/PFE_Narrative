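; BP_DownFlamePoint is a flame point actor whose logic drops the player's life to a lower flame tier.
; Its DoOnce-gated chain disables the cube, stops timers on cached flame zones and points, then re-enables it after a timeline.
; As wired, begin overlap is empty, the DoOnce entry is unreachable, and the end-overlap life-reset timeline sits behind an always-false branch.
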(event `self.ReceiveBeginPlay`
  (bind _returnvalue (`GameplayStatics.GetActorOfClass` "/Game/Blueprints/Player/BP_Player.BP_Player_C"))
  (set `self.PlayerRef` _returnvalue)
  (bind _outactors (`GameplayStatics.GetAllActorsOfClass` "/Game/Blueprints/Zones/BP_DownFlameZone.BP_DownFlameZone_C"))
  (set `self.DownZonesArray` _outactors)
  (bind _outactors_2 (`GameplayStatics.GetAllActorsOfClass` "/Game/Blueprints/Zones/BP_UpFlameZone.BP_UpFlameZone_C"))
  (set `self.UpZonesArray` _outactors_2)
  (bind _outactors_3 (`GameplayStatics.GetAllActorsOfClass` "/Game/Blueprints/Zones/BP_UpFlamePoint.BP_UpFlamePoint_C"))
  (set `self.UpPointsArray` _outactors_3)
  (bind _outactors_4 (`GameplayStatics.GetAllActorsOfClass` "BP_DownFlamePoint_C"))
  (set `self.DownPoint` _outactors_4))

(event `self.ReceiveActorBeginOverlap`
  (params (OtherActor :type "Actor Object Reference")))

(event `ResetDoOnce`
  (bind _cube (`self.Cube`))
  (bind _cube_2 (`self.Cube`))
  (`/Engine/EditorBlueprintResources/StandardMacros.DoOnce` false :!via `Reset`
    (:`Completed`
      (cast `/Game/Blueprints/Player/BP_Player` (stale `self.ReceiveActorBeginOverlap` OtherActor))
      (`self.ChangePlayerState`)
      (`PrimitiveComponent.SetCollisionEnabled` _cube_2 "NoCollision")
      (`PrimitiveComponent.SetMaterial` _cube_2 0 "/Game/Materials/M_DisabledPoint.M_DisabledPoint")
      (for _array_element (`self.DownZonesArray`)
        (`/Game/Blueprints/Zones/BP_DownFlameZone.StopTimer` _array_element))
      (for _array_element_2 (`self.UpZonesArray`)
        (`/Game/Blueprints/Zones/BP_UpFlameZone.Stop` _array_element_2)
        (for _array_element_3 (`self.UpPointsArray`)
          (`/Game/Blueprints/Zones/BP_UpFlamePoint.StopTimer` _array_element_3)
          (for _array_element_4 (`self.DownPoint`)
            (`self.StopTimerDown` _array_element_4))
          (`Timeline|TimBeforeEnable` :!via `PlayFromStart`
            (:`Finished`
              (`PrimitiveComponent.SetCollisionEnabled` _cube "QueryOnly")
              (`PrimitiveComponent.SetMaterial` _cube 0 "/Game/Materials/M_Point-.M_Point-")
              (`self.ResetDoOnce`))))))))

(event `ChangePlayerState`
  (bind _playerref (`self.PlayerRef`))
  (bind _playerref_2 (`self.PlayerRef`))
  (bind _playerref_3 (`self.PlayerRef`))
  (bind _playerlife (`/Game/Blueprints/Player/BP_Player.PlayerLife` (`self.PlayerRef`)))
  (if (`KismetMathLibrary.InRange_IntInt` _playerlife 0 30 false)
    (set `/Game/Blueprints/Player/BP_Player.PlayerLife` 0 _playerref)
    (`/Game/Blueprints/Player/BP_Player.CheckPlayerLife` _playerref)
    (elif (`KismetMathLibrary.InRange_IntInt` _playerlife 30 70 false)
      (set `/Game/Blueprints/Player/BP_Player.PlayerLife` (`self.SmallFlameHP`) _playerref_2)
      (`/Game/Blueprints/Player/BP_Player.CheckPlayerLife` _playerref_2)
      (elif (`KismetMathLibrary.InRange_IntInt` _playerlife 70 100 false)
        (set `/Game/Blueprints/Player/BP_Player.PlayerLife` (`self.DefaultFlameHP`) _playerref_3)
        (`/Game/Blueprints/Player/BP_Player.CheckPlayerLife` _playerref_3)))))

(event `self.ReceiveActorEndOverlap`
  (params (OtherActor :type "Actor Object Reference"))
  (bind _playerref (`self.PlayerRef`))
  (`|ExecutionSequence`
    (:`then_0`
      (`Timeline|Check`))
    (:`then_1`
      (if (not true)
        (`Timeline|Timeline` :!via `PlayFromStart` :!label _label
          (:`Finished`
            (set `/Game/Blueprints/Player/BP_Player.PlayerLife` 50 _playerref)
            (`/Game/Blueprints/Player/BP_Player.CheckPlayerLife` _playerref)
            (`self.ResetDoOnce`)))))))

(event `StopTimerDown`
  (goto _label :!via `Stop`))

(fn `UserConstructionScript`)