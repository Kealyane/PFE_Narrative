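; Test drop variant of a one-shot flame zone that travels along an InterpToMovement path, showing big-fire sprites when its effect is INCREASE.
; Movement starts after a random delay; on each stop the actor snaps to the first control point and restarts after another.
; A PFECharacter overlap deactivates the Cube, then a second later swaps it to a disabled material and ignores pawns until DisableDuration elapses.
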(event `self.ReceiveBeginPlay`
  (`self.InitSoundComponent` (`self.Sound`))
  (`KismetSystemLibrary.Delay` (`KismetMathLibrary.RandomFloatInRange` 0.1 1.0))
  (`ActorComponent.Activate` (`self.InterpToMovement`) false)
  (if (`|EnumEquality` (`self.ZoneEffect`) "INCREASE")
    (`PaperSpriteComponent.SetSprite` (`self.PaperSprite2`) "/Game/Sprites/Decor/BigFire_Sprite_0.BigFire_Sprite_0")
    (`PaperSpriteComponent.SetSprite` (`self.PaperSprite`) "/Game/Sprites/Decor/BigFire_Sprite_1.BigFire_Sprite_1")
    (`PaperSpriteComponent.SetSprite` (`self.PaperSprite1`) "/Game/Sprites/Decor/BigFire_Sprite_3.BigFire_Sprite_3")))

(event `self.ReceiveActorBeginOverlap`
  (params (OtherActor :type "Actor Object Reference"))
  (cast `PFECharacter` OtherActor)
  (`ActorComponent.SetActive` (`self.Cube`) false false)
  (`KismetSystemLibrary.Delay` 1.0)
  (`PrimitiveComponent.SetMaterial` (`self.Cube`) 0 "/Game/Materials/M_DisabledPoint.M_DisabledPoint")
  (`PrimitiveComponent.SetCollisionResponseToChannel` (`self.Cube`) "ECC_Pawn" "ECR_Ignore")
  (`KismetSystemLibrary.Delay` (`self.DisableDuration`))
  (`PrimitiveComponent.SetMaterial` (`self.Cube`) 0 "/Game/Materials/M_Point-.M_Point-")
  (`PrimitiveComponent.SetCollisionResponseToChannel` (`self.Cube`) "ECC_Pawn" "ECR_Overlap")
  (`ActorComponent.SetActive` (`self.Cube`) true false))

(event `self.InterpToMovement.OnInterpToStop`
  (params (ImpactResult :type "HitResult Structure (by ref)") (Time :type "Float (single-precision)"))
  (bind _output_positioncontrolpoint (break `InterpControlPoint` (`|GetArrayItem` (`InterpToMovementComponent.ControlPoints` (`self.InterpToMovement`)))))
  (`self.K2_SetActorLocation` _output_positioncontrolpoint)
  (`KismetSystemLibrary.Delay` (`KismetMathLibrary.RandomFloatInRange` 0.2 1.0))
  (`ActorComponent.Activate` (`self.InterpToMovement`) false))

(fn `UserConstructionScript`)