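; One-shot trigger zone, named for decreasing flame, that switches off when a PFECharacter enters and later respawns; no flame change happens in this graph.
; On overlap, a DoOnce gate plays the off sound, ignores the Pawn channel and hides the flipbook.
; After one second plus DisableDuration, Respawn resets the gate through Reboot, restores overlap, plays the on sound and shows the flipbook.
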(event `self.ReceiveBeginPlay`
  (`self.InitSoundComponent` (`self.Sound`)))

(event `self.ReceiveActorBeginOverlap`
  (params (OtherActor :type "Actor Object Reference"))
  (bind _audio (`self.Audio`))
  (cast `PFECharacter` OtherActor)
  (`/Engine/EditorBlueprintResources/StandardMacros.DoOnce` false :!label _label
    (:`Completed`
      (`AudioComponent.SetSound` _audio (`self.SoundOff`))
      (`AudioComponent.Play` _audio 0.0)
      (`PrimitiveComponent.SetCollisionResponseToChannel` (`self.Trigger`) "ECC_Pawn" "ECR_Ignore")
      (`SceneComponent.SetVisibility` (`self.PaperFlipbook`) false false)
      (`KismetSystemLibrary.Delay` 1.0)
      (`KismetSystemLibrary.Delay` (`self.DisableDuration`))
      (`self.Respawn`))))

(event `Reboot`
  (goto _label :!via `Reset`))

(event `Respawn`
  (bind _audio (`self.Audio`))
  (`|ExecutionSequence`
    (:`then_0`
      (`self.Reboot`)
      (`PrimitiveComponent.SetCollisionResponseToChannel` (`self.Trigger`) "ECC_Pawn" "ECR_Overlap")
      (`AudioComponent.SetSound` _audio (`self.SoundOn`))
      (`AudioComponent.Play` _audio 0.0))
    (:`then_1`
      (`SceneComponent.SetVisibility` (`self.PaperFlipbook`) true false))))

(fn `UserConstructionScript`)