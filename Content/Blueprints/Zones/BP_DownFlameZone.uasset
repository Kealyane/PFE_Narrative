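; BP_DownFlameZone is a zone that periodically lowers the player's flame while BP_Player is inside.
; BeginPlay caches the player, flame zones and points, and sets the player's flame amount.
; Entering flags the player as in a zone, starts a looping LowerFlame timer and stops the others' timers or timelines.
; Exiting clears the timer and uses CanExit and BackToMid timelines for the zone flag and conditional life reset to midpoint.
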(event `self.ReceiveBeginPlay`
  (bind _returnvalue (`GameplayStatics.GetActorOfClass` "/Game/Blueprints/Player/BP_Player.BP_Player_C"))
  (set `self.PlayerRef` _returnvalue)
  (set `/Game/Blueprints/Player/BP_Player.FlameAmountToAddOrTake` (`self.FlameAmountToTakePerSecond`) _returnvalue)
  (bind _outactors (`GameplayStatics.GetAllActorsOfClass` "/Game/Blueprints/Zones/BP_UpFlameZone.BP_UpFlameZone_C"))
  (set `self.ZoneUpRef` _outactors)
  (bind _outactors_2 (`GameplayStatics.GetAllActorsOfClass` "/Game/Blueprints/Zones/BP_DownFlamePoint.BP_DownFlamePoint_C"))
  (set `self.DownPointsArray` _outactors_2)
  (bind _outactors_3 (`GameplayStatics.GetAllActorsOfClass` "/Game/Blueprints/Zones/BP_UpFlamePoint.BP_UpFlamePoint_C"))
  (set `self.UpPointsArray` _outactors_3)
  (bind _outactors_4 (`GameplayStatics.GetAllActorsOfClass` "BP_DownFlameZone_C"))
  (set `self.DowZoneArray` _outactors_4))

(event `self.ReceiveActorBeginOverlap`
  (params (OtherActor :type "Actor Object Reference"))
  (bind _asbp_player (cast `/Game/Blueprints/Player/BP_Player` OtherActor))
  (set `/Game/Blueprints/Player/BP_Player.IsInAZone?` true _asbp_player)
  (bind _returnvalue (`KismetSystemLibrary.K2_SetTimerDelegate` (delegate `LowerFlame`) (`self.TimeBetweenChecks`) true))
  (set `self.TimerByHandle` _returnvalue)
  (for _array_element (`self.ZoneUpRef`)
    (`/Game/Blueprints/Zones/BP_UpFlameZone.Stop` _array_element))
  (for _array_element_2 (`self.UpPointsArray`)
    (`/Game/Blueprints/Zones/BP_UpFlamePoint.StopTimer` _array_element_2))
  (for _array_element_3 (`self.DownPointsArray`)
    (`/Game/Blueprints/Zones/BP_DownFlamePoint.StopTimerDown` _array_element_3))
  (for _array_element_4 (`self.DowZoneArray`)
    (`self.StopTimer` _array_element_4)))

(event `LowerFlame`
  (bind _playerref (`self.PlayerRef`))
  (`/Game/Blueprints/Player/BP_Player.LowerFlame` _playerref)
  (`KismetSystemLibrary.PrintString` (`KismetStringLibrary.Conv_IntToString` (`/Game/Blueprints/Player/BP_Player.PlayerLife` _playerref))))

(event `Stop`
  (`Timeline|CanExit ?` :!via `Stop` :!label _label
    (:`Finished`
      (set `/Game/Blueprints/Player/BP_Player.IsInAZone?` false (`self.PlayerRef`)))))

(event `self.ReceiveActorEndOverlap`
  (params (OtherActor :type "Actor Object Reference"))
  (bind _playerref (`self.PlayerRef`))
  (`|ExecutionSequence`
    (:`then_0`
      (goto _label :!via `PlayFromStart`))
    (:`then_1`
      (`KismetSystemLibrary.K2_ClearAndInvalidateTimerHandle` (`self.TimerByHandle`))
      (if (not (`/Game/Blueprints/Player/BP_Player.IsInAZone?` (`self.PlayerRef`)))
        (`Timeline|BackToMid` :!via `PlayFromStart` :!label _label_2
          (:`Finished`
            (set `/Game/Blueprints/Player/BP_Player.PlayerLife` 50 _playerref)
            (`/Game/Blueprints/Player/BP_Player.CheckPlayerLife` _playerref)))))))

(event `StopTimer`
  (goto _label_2 :!via `Stop`))

(fn `UserConstructionScript`)