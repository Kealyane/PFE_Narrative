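; BP_UpFlameZone is a zone actor that reacts to BP_Player overlap and manages the player's flame-based life.
; BeginPlay passes a per-second flame amount to the player and caches all down zones plus up and down points.
; Entering stops the BackToNormal timeline, starts a looping timer with no visible bound event, and halts those actors' timers.
; Leaving clears the timer and replays BackToNormal, which resets player life to 50 on finishing.
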(event `self.ReceiveBeginPlay`
  (bind _returnvalue (`GameplayStatics.GetActorOfClass` "/Game/Blueprints/Player/BP_Player.BP_Player_C"))
  (set `self.PlayerRef` _returnvalue)
  (set `/Game/Blueprints/Player/BP_Player.FlameAmountToAddOrTake` (`self.FlameAmountToTakePerSecond`) _returnvalue)
  (bind _outactors (`GameplayStatics.GetAllActorsOfClass` "/Game/Blueprints/Zones/OLD/BP_DownFlameZone.BP_DownFlameZone_C"))
  (set `self.DownZoneRef` _outactors)
  (bind _outactors_2 (`GameplayStatics.GetAllActorsOfClass` "/Game/Blueprints/Zones/OLD/BP_DownFlamePoint.BP_DownFlamePoint_C"))
  (set `self.DownPointsArray` _outactors_2)
  (bind _outactors_3 (`GameplayStatics.GetAllActorsOfClass` "/Game/Blueprints/Zones/OLD/BP_UpFlamePoint.BP_UpFlamePoint_C"))
  (set `self.UpPointsArray` _outactors_3))

(event `self.ReceiveActorBeginOverlap`
  (params (OtherActor :type "Actor Object Reference"))
  (cast `/Game/Blueprints/Player/BP_Player` OtherActor)
  (`KismetSystemLibrary.PrintString` "Hello" true true (struct :`R` 1.0 :`G` 0.141743 :`A` 1.0))
  (`self.Stop`)
  (bind _returnvalue (`KismetSystemLibrary.K2_SetTimerDelegate` :`Time` (`self.TimeBetweenChecks`) :`bLooping` true))
  (set `self.TimerByHandle` _returnvalue)
  (for _array_element (`self.DownZoneRef`)
    (`/Game/Blueprints/Zones/OLD/BP_DownFlameZone.StopTimer` _array_element))
  (for _array_element_2 (`self.UpPointsArray`)
    (`/Game/Blueprints/Zones/OLD/BP_UpFlamePoint.StopTimer` _array_element_2))
  (for _array_element_3 (`self.DownPointsArray`)
    (`/Game/Blueprints/Zones/OLD/BP_DownFlamePoint.StopTimerDown` _array_element_3)))

(event `self.ReceiveActorEndOverlap`
  (params (OtherActor :type "Actor Object Reference"))
  (bind _playerref (`self.PlayerRef`))
  (`KismetSystemLibrary.K2_ClearAndInvalidateTimerHandle` (`self.TimerByHandle`))
  (`Timeline|BackToNormal` :!via `PlayFromStart` :!label _label
    (:`Finished`
      (set `/Game/Blueprints/Player/BP_Player.PlayerLife` 50 _playerref)
      (`/Game/Blueprints/Player/BP_Player.CheckPlayerLife` _playerref))))

(event `Stop`
  (goto _label :!via `Stop`))

(fn `UserConstructionScript`)