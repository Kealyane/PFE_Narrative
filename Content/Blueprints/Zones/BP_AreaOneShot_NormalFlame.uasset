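; One-shot flame zone that temporarily switches itself off when a PFECharacter overlaps it, then re-arms.
; BeginPlay initializes the sound component with Sound.
; On overlap the flipbook hides immediately, and one second later the Cube takes the disabled material and ignores Pawns.
; After DisableDuration, the Cube's point material and Pawn overlap response return and the flipbook shows again.
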(event `self.ReceiveBeginPlay`
  (`self.InitSoundComponent` (`self.Sound`)))

(event `self.ReceiveActorBeginOverlap`
  (params (OtherActor :type "Actor Object Reference"))
  (bind _paperflipbook (`self.PaperFlipbook`))
  (cast `PFECharacter` OtherActor)
  (`|ExecutionSequence`
    (:`then_0`
      (`KismetSystemLibrary.Delay` 1.0)
      (`PrimitiveComponent.SetMaterial` (`self.Cube`) 0 "/Game/Materials/M_DisabledPoint.M_DisabledPoint")
      (`PrimitiveComponent.SetCollisionResponseToChannel` (`self.Cube`) "ECC_Pawn" "ECR_Ignore")
      (`KismetSystemLibrary.Delay` (`self.DisableDuration`))
      (`|ExecutionSequence`
        (:`then_0`
          (`PrimitiveComponent.SetMaterial` (`self.Cube`) 0 "/Game/Materials/M_Point+.M_Point+")
          (`PrimitiveComponent.SetCollisionResponseToChannel` (`self.Cube`) "ECC_Pawn" "ECR_Overlap"))
        (:`then_1`
          (`SceneComponent.SetVisibility` _paperflipbook true false))))
    (:`then_1`
      (`SceneComponent.SetVisibility` _paperflipbook false false))))

(fn `UserConstructionScript`)