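; BP_UpFlameZone is a zone that raises the player's flame while BP_Player overlaps it.
; On BeginPlay it caches the player and overwrites its FlameAmountToAddOrTake, then a looping timer started on overlap calls IncreaseFlame on the player.
; Any end overlap, unfiltered by actor, clears the timer and plays the BackToDefault timeline, which lerps PlayerLife toward 50 and rechecks it each update.
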(event `self.ReceiveBeginPlay`
  (bind _returnvalue (`GameplayStatics.GetActorOfClass` "/Game/Blueprints/Player/BP_Player.BP_Player_C"))
  (set `self.PlayerRef` _returnvalue)
  (set `/Game/Blueprints/Player/BP_Player.FlameAmountToAddOrTake` (`self.FlameAmountToTakePerSecond`) _returnvalue))

(event `self.ReceiveActorBeginOverlap`
  (params (OtherActor :type "Actor Object Reference"))
  (cast `/Game/Blueprints/Player/BP_Player` OtherActor)
  (`KismetSystemLibrary.PrintString` "Hello")
  (bind _returnvalue (`KismetSystemLibrary.K2_SetTimerDelegate` (delegate `IncreaseFlame`) (`self.TimeBetweenChecks`) true))
  (set `self.TimerByHandle` _returnvalue))

(event `IncreaseFlame`
  (bind _playerref (`self.PlayerRef`))
  (`/Game/Blueprints/Player/BP_Player.IncreaseFlame` _playerref)
  (`KismetSystemLibrary.PrintString` (`KismetStringLibrary.Conv_IntToString` (`/Game/Blueprints/Player/BP_Player.PlayerLife` _playerref))))

(event `self.ReceiveActorEndOverlap`
  (params (OtherActor :type "Actor Object Reference"))
  (bind _playerref (`self.PlayerRef`))
  (`KismetSystemLibrary.K2_ClearAndInvalidateTimerHandle` (`self.TimerByHandle`))
  (bind (_direction _backtodefault) (`Timeline|BackToDefault`)
    (:`Update`
      (set `/Game/Blueprints/Player/BP_Player.PlayerLife` (`KismetMathLibrary.FTrunc` (`KismetMathLibrary.Lerp` (`KismetMathLibrary.Conv_IntToDouble` (`/Game/Blueprints/Player/BP_Player.PlayerLife` _playerref)) 50.0 _backtodefault)) _playerref)
      (`/Game/Blueprints/Player/BP_Player.CheckPlayerLife` _playerref))))

(fn `UserConstructionScript`)