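; Torch path actor that lights a timed trail of fire flipbooks and orange point lights along its spline's points, then puts it out.
; BeginPlay caches the spline points; TriggerLights switches to UI-only input while spawning components one by one through a DelayedForLoop macro.
; It then restores game input, pauses briefly, and LightsOut destroys them in the same order before reactivating its AffiliatedTrigger.
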(event `self.ReceiveBeginPlay`
  (bind _spline (`self.Spline`))
  (for _index (range (`SplineComponent.GetNumberOfSplinePoints` _spline))
    (`KismetArrayLibrary.Array_Add` (`self.SplinePoints`) (`SplineComponent.GetSplinePointAt` _spline _index "Local"))))

(event `TriggerLights`
  (bind (_lightpos_x _lightpos_y _lightpos_z) (`KismetMathLibrary.BreakVector` (`self.LightPos`)))
  (`WidgetBlueprintLibrary.SetInputMode_UIOnlyEx` (`GameplayStatics.GetPlayerController` 0) null "DoNotLock" true)
  (bind _arrayelement (`self.DelayedForLoop` (`self.DelayInbetweenAppear`) (`self.SplinePoints`))
    (:`Loop`
      (bind _output_get (set `self.LightPos` (`.Position` (break `SplinePoint` _arrayelement))))
      (bind _returnvalue (`AddComponent|NODE_AddPaperFlipbookComponent-0` :`RelativeTransform` (`KismetMathLibrary.MakeTransform` _output_get)))
      (set `self.PointFlipbook` _returnvalue)
      (`PaperFlipbookComponent.SetFlipbook` _returnvalue "/Game/Sprites/Decor/FB_Fire.FB_Fire")
      (`SceneComponent.SetVisibility` _returnvalue true false)
      (`KismetArrayLibrary.Array_Add` (`self.SplineFlipbookArray`) _returnvalue)
      (bind _returnvalue_2 (`AddComponent|NODE_AddPointLightComponent-3` :`RelativeTransform` (`KismetMathLibrary.MakeTransform` (`KismetMathLibrary.MakeVector` _lightpos_x (+ _lightpos_y 15.0) (- _lightpos_z 300.0)))))
      (`LightComponent.SetLightColor` _returnvalue_2 (struct :`R` 1.0 :`G` 0.526792 :`A` 1.0) true)
      (`LightComponent.SetIntensity` _returnvalue_2 20000.0)
      (bind _output_get_2 (set `self.PointLight` _returnvalue_2))
      (`KismetArrayLibrary.Array_Add` (`self.SplineLightsArray`) _output_get_2))
    (:`Completed`
      (`WidgetBlueprintLibrary.SetInputMode_GameOnly` (`GameplayStatics.GetPlayerController` 0))
      (`KismetSystemLibrary.Delay` 2.0)
      (`self.LightsOut`))))

(event `LightsOut`
  (bind _arrayelement (`self.DelayedForLoop` (`self.DelayInbetweenAppear`) (`self.SplineFlipbookArray`))
    (:`Loop`
      (`ActorComponent.K2_DestroyComponent` _arrayelement)
      (`ActorComponent.K2_DestroyComponent` (`|GetArrayItem` (`self.SplineLightsArray`) (`self.PointLightToDelete`)))
      (`/Engine/EditorBlueprintResources/StandardMacros.IncrementInt` (`self.PointLightToDelete`)))
    (:`Completed`
      (`KismetArrayLibrary.Array_Clear` (`self.SplineFlipbookArray`))
      (`KismetArrayLibrary.Array_Clear` (`self.SplineLightsArray`))
      (set `self.PointLightToDelete` 0)
      (`/Game/Blueprints/Level/BP_TorchPathTrigger.Reactivate` (`self.AffiliatedTrigger`)))))

(fn `UserConstructionScript`)