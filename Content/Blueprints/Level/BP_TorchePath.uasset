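; Torch path actor that lights a trail of fire sprites along a spline when TriggerLights is called, then clears it.
; BeginPlay caches the spline's local-space points.
; TriggerLights uses a custom DelayedForLoop macro, a for-each with a delay between iterations, to spawn a fire Paper Sprite component at each point in turn.
; After a short pause, a second delayed loop destroys the sprites in the same order.
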(event `self.ReceiveBeginPlay`
  (bind _spline (`self.Spline`))
  (for _index (range (`SplineComponent.GetNumberOfSplinePoints` _spline))
    (`KismetArrayLibrary.Array_Add` (`self.SplinePoints`) (`SplineComponent.GetSplinePointAt` _spline _index "Local"))))

(event `TriggerLights`
  (bind _arrayelement (`self.DelayedForLoop` 1.0 (`self.SplinePoints`))
    (:`Loop`
      (bind _returnvalue (`AddComponent|NODE_AddPaperSpriteComponent-3` :`RelativeTransform` (`KismetMathLibrary.MakeTransform` (`.Position` (break `SplinePoint` _arrayelement)))))
      (set `self.PlcaholderPoint` _returnvalue)
      (`PaperSpriteComponent.SetSprite` _returnvalue "/Game/Sprites/Decor/BigFire_Sprite_4.BigFire_Sprite_4")
      (`SceneComponent.SetVisibility` _returnvalue true false)
      (`KismetArrayLibrary.Array_Add` (`self.SplinePlacholder`) _returnvalue))
    (:`Completed`
      (`KismetSystemLibrary.Delay` 1.0)
      (bind _arrayelement_2 (`self.DelayedForLoop` (`self.DelayInbetweenAppearDisappear`) (`self.SplinePlacholder`))
        (:`Loop`
          (`ActorComponent.K2_DestroyComponent` _arrayelement_2))))))

(fn `UserConstructionScript`)