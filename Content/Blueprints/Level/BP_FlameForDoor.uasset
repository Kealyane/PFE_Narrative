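; A flame brazier that the player lights to contribute toward opening an affiliated door.
; On overlap with the player, it checks that the player's flame value exceeds 30.
; If so, it shows its own flame, increments the door's activated flame count and has the door re-check its flames.
; Nothing guards against repeat overlaps, so each qualifying overlap increments the count again.
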(event `self.ReceiveActorBeginOverlap`
  (params (OtherActor :type "Actor Object Reference"))
  (bind _affiliateddoor (`self.AffiliatedDoor`))
  (bind _asbp_player (cast `/Game/Blueprints/Player/BP_Player` OtherActor))
  (if (not (<= (`FlameComponent.GetFlameValue` (`/Game/Blueprints/Player/BP_Player.Flame` _asbp_player)) 30.0))
    (`SceneComponent.SetVisibility` (`self.Flame`) true false)
    (`/Engine/EditorBlueprintResources/StandardMacros.IncrementInt` (`/Game/Blueprints/Level/BP_FlameDoor.ActivatedFlames` _affiliateddoor)
      (:`  `
        (`/Game/Blueprints/Level/BP_FlameDoor.CheckFlames` _affiliateddoor)))))

(fn `UserConstructionScript`)