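; Level transition trigger actor that sends the player to a configured next level.
; When a PFECharacter overlaps its box, it fades out the music and calls ScreenFadeIn on the existing WBP_FadeScreen widget.
; It saves NextLevel through BP_PFEGameInstance, then after a short delay opens that level by the path the game instance resolves.
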(event `self.ReceiveBeginPlay`
  (bind _asbp_pfegame_instance (cast `/Game/Blueprints/Core/BP_PFEGameInstance` (`GameplayStatics.GetGameInstance`)))
  (set `self.PFEGameInstance` _asbp_pfegame_instance))

(event `self.Box.OnComponentBeginOverlap`
  (params (OverlappedComponent :type "PrimitiveComponent Object Reference") (OtherActor :type "Actor Object Reference") (OtherComp :type "PrimitiveComponent Object Reference") (OtherBodyIndex :type Integer) (bFromSweep :type Boolean) (SweepResult :type "HitResult Structure (by ref)"))
  (cast `PFECharacter` OtherActor)
  (`self.FadeInMusicScreen`)
  (bind _asbp_pfegame_instance (cast `/Game/Blueprints/Core/BP_PFEGameInstance` (`GameplayStatics.GetGameInstance`)))
  (`/Game/Blueprints/Core/BP_PFEGameInstance.SaveLevel` _asbp_pfegame_instance (`self.NextLevel`))
  (`KismetSystemLibrary.Delay` 1.5)
  (`self.OpenNextLevel`))

(fn `FadeInMusicScreen`
  (`AudioComponent.FadeOut` (`AmbientSound.AudioComponent` (`self.Music`)) 0.8 0.0 "Linear")
  (bind _foundwidgets (`WidgetBlueprintLibrary.GetAllWidgetsOfClass` "/Game/UI/Widgets/HUD/WBP_FadeScreen.WBP_FadeScreen_C"))
  (`/Game/UI/Widgets/HUD/WBP_FadeScreen.ScreenFadeIn` (`|GetArrayItem` _foundwidgets)))

(fn `OpenNextLevel`
  (bind _levelpath (`/Game/Blueprints/Core/BP_PFEGameInstance.GetLevelPath` (`self.PFEGameInstance`) (`self.NextLevel`)))
  (`GameplayStatics.OpenLevel` (`KismetStringLibrary.Conv_StringToName` _levelpath)))

(fn `UserConstructionScript`)