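; Trigger sphere for a torch path that lights the path when BP_Player enters.
; On BeginPlay it registers itself with its AffiliatedPath; a DoOnce then limits overlap to one TriggerLights call and hides the sphere.
; Reactivate shows the sphere again and resets that gate.
; CanLightsOut resets a second DoOnce leading to LightsOut, but the exit logic that enters it and clears IsInTrigger is disconnected.
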(event `self.ReceiveBeginPlay`
  (set `/Game/Blueprints/Level/Torches/BP_TorchPath.AffiliatedTrigger` self (`self.AffiliatedPath`)))

(event `self.ReceiveActorBeginOverlap`
  (params (OtherActor :type "Actor Object Reference"))
  (cast `/Game/Blueprints/Player/BP_Player` OtherActor)
  (`/Engine/EditorBlueprintResources/StandardMacros.DoOnce` false :!label _label
    (:`Completed`
      (`SceneComponent.SetVisibility` (`self.Sphere`) false false)
      (set `self.IsInTrigger` true)
      (`/Game/Blueprints/Level/Torches/BP_TorchPath.TriggerLights` (`self.AffiliatedPath`)))))

(event `Reactivate`
  (`SceneComponent.SetVisibility` (`self.Sphere`) true false)
  (goto _label :!via `Reset`))

(event `self.ReceiveActorEndOverlap`
  (params (OtherActor :type "Actor Object Reference")))

(event `CanLightsOut`
  (`/Engine/EditorBlueprintResources/StandardMacros.DoOnce` true :!via `Reset`
    (:`Completed`
      (`/Game/Blueprints/Level/Torches/BP_TorchPath.LightsOut` (`self.AffiliatedPath`)))))

(fn `UserConstructionScript`)