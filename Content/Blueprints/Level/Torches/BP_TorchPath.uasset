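; Spline-based torch path that lights up and goes out one point at a time.
; BeginPlay caches the spline points.
; TriggerLights uses a delayed-loop macro to add a fire flipbook and orange point light at each point, plus spawn a BP_LightSphere.
; LightsOut removes them in the same staggered order, clears the arrays and reactivates the affiliated trigger.
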(event `self.ReceiveBeginPlay`
  (bind _spline (`self.Spline`))
  (for _index (range (`SplineComponent.GetNumberOfSplinePoints` _spline))
    (`KismetArrayLibrary.Array_Add` (`self.SplinePoints`) (`SplineComponent.GetSplinePointAt` _spline _index "Local"))))

(event `TriggerLights`
  (bind (_lightpos_x _lightpos_y _lightpos_z) (`KismetMathLibrary.BreakVector` (`self.LightPos`)))
  (bind (_returnvalue_x _returnvalue_y _returnvalue_z) (`KismetMathLibrary.BreakVector` (`SceneComponent.K2_GetComponentLocation` (`self.PointFlipbook`))))
  (bind _arrayelement (`self.DelayedForLoop` (`self.DelayInbetweenAppear`) (`self.SplinePoints`))
    (:`Loop`
      (bind _output_get (set `self.LightPos` (`.Position` (break `SplinePoint` _arrayelement))))
      (bind _returnvalue (`AddComponent|NODE_AddPaperFlipbookComponent-0` :`RelativeTransform` (`KismetMathLibrary.MakeTransform` _output_get)))
      (set `self.PointFlipbook` _returnvalue)
      (`PaperFlipbookComponent.SetFlipbook` _returnvalue "/Game/Sprites/Decor/FB_Fire.FB_Fire")
      (`SceneComponent.SetVisibility` _returnvalue true false)
      (`KismetArrayLibrary.Array_Add` (`self.SplineFlipbookArray`) _returnvalue)
      (bind _returnvalue_2 (`AddComponent|NODE_AddPointLightComponent-3` :`RelativeTransform` (`KismetMathLibrary.MakeTransform` (`KismetMathLibrary.MakeVector` _lightpos_x (+ _lightpos_y 15.0) (- _lightpos_z 100.0)))))
      (`LightComponent.SetLightColor` _returnvalue_2 (struct :`R` 1.0 :`G` 0.526792 :`A` 1.0) true)
      (`LightComponent.SetIntensity` _returnvalue_2 1000.0)
      (bind _output_get_2 (set `self.PointLight` _returnvalue_2))
      (`KismetArrayLibrary.Array_Add` (`self.SplineLightsArray`) _output_get_2)
      (bind _returnvalue_3 (`|SpawnActorFromClass` "/Game/Blueprints/Level/Torches/BP_LightSphere.BP_LightSphere_C" (`KismetMathLibrary.MakeTransform` (`KismetMathLibrary.MakeVector` _returnvalue_x (+ _returnvalue_y 100.0) (- _returnvalue_z 100.0))) "AlwaysSpawn" "MultiplyWithRoot" null null))
      (`KismetArrayLibrary.Array_Add` (`self.SphereArray`) _returnvalue_3))))

(event `LightsOut`
  (bind _arrayelement (`self.DelayedForLoop` (`self.DelayInbetweenAppear`) (`self.SplineFlipbookArray`))
    (:`Loop`
      (`ActorComponent.K2_DestroyComponent` _arrayelement)
      (`ActorComponent.K2_DestroyComponent` (`|GetArrayItem` (`self.SplineLightsArray`) (`self.PointLightToDelete`)))
      (`self.K2_DestroyActor` (`|GetArrayItem` (`self.SphereArray`) (`self.PointLightToDelete`)))
      (`/Engine/EditorBlueprintResources/StandardMacros.IncrementInt` (`self.PointLightToDelete`)))
    (:`Completed`
      (`KismetArrayLibrary.Array_Clear` (`self.SplineFlipbookArray`))
      (`KismetArrayLibrary.Array_Clear` (`self.SplineLightsArray`))
      (`KismetArrayLibrary.Array_Clear` (`self.SphereArray`))
      (set `self.PointLightToDelete` 0)
      (`/Game/Blueprints/Level/Torches/BP_TorchPathTrigger.Reactivate` (`self.AffiliatedTrigger`)))))

(fn `UserConstructionScript`)