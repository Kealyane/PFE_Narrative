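; BP_TorchPathTrigger is a box trigger that lights an affiliated torch path when the player walks into it.
; On BeginPlay it registers itself as the path's AffiliatedTrigger.
; An overlap with BP_Player calls TriggerLights on the path and disables the box collision, so it fires once until Reactivate restores query-only collision.
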(event `self.ReceiveBeginPlay`
  (set `/Game/Blueprints/Level/BP_TorchPath.AffiliatedTrigger` self (`self.AffiliatedPath`)))

(event `self.ReceiveActorBeginOverlap`
  (params (OtherActor :type "Actor Object Reference"))
  (cast `/Game/Blueprints/Player/BP_Player` OtherActor)
  (`/Game/Blueprints/Level/BP_TorchPath.TriggerLights` (`self.AffiliatedPath`))
  (`PrimitiveComponent.SetCollisionEnabled` (`self.Box`) "NoCollision"))

(event `Reactivate`
  (`PrimitiveComponent.SetCollisionEnabled` (`self.Box`) "QueryOnly"))

(fn `UserConstructionScript`)