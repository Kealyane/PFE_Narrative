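; Boss NPC actor that displays Paper2D flipbook animations for idling, yelling and walking.
; BeginPlay picks Yell or Idle from IsYelling, while custom events swap the flipbook, with both walk directions using BossWalkRight.
; MakeFlamesAppear forwards to the BP_Player found in the level.
; Insult and HideInsults are empty, leaving the speech-bubble visibility and angry sound logic disconnected.
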(event `self.ReceiveBeginPlay`
  (if (`self.IsYelling`)
    (`self.Yell`)
    (else
      (`self.Idle`))))

(event `WalkLeft`
  (`PaperFlipbookComponent.SetFlipbook` (`self.PaperFlipbook`) "/Game/Characters/Boss/Flipbooks/BossWalkRight.BossWalkRight"))

(event `WalkRight`
  (`PaperFlipbookComponent.SetFlipbook` (`self.PaperFlipbook`) "/Game/Characters/Boss/Flipbooks/BossWalkRight.BossWalkRight"))

(event `Yell`
  (`PaperFlipbookComponent.SetFlipbook` (`self.PaperFlipbook`) "/Game/Characters/Boss/Flipbooks/BossYell.BossYell"))

(event `Idle`
  (`PaperFlipbookComponent.SetFlipbook` (`self.PaperFlipbook`) "/Game/Characters/Boss/Flipbooks/BossIdle.BossIdle"))

(event `Insult`)

(event `HideInsults`)

(event `MakeFlamesAppear`
  (bind _returnvalue (`GameplayStatics.GetActorOfClass` "/Game/Blueprints/Player/BP_Player.BP_Player_C"))
  (`/Game/Blueprints/Player/BP_Player.MakeFlamesAppear` _returnvalue))

(fn `UserConstructionScript`)