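; BP_NewBoss is a flipbook-animated boss NPC whose events are not called within this graph.
; Walk, idle and yell events swap flipbooks, with both walk directions using BossWalkRight.
; Yell also plays a sound and sets WasShoved on BP_Player, StopYell clears it, and MakeFlamesAppear forwards to the player.
; Insult is empty, and the insult bubble visibility toggles are disconnected.
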(event `WalkLeft`
  (`PaperFlipbookComponent.SetFlipbook` (`self.PaperFlipbook`) "/Game/Sprites/NPC/Boss/WalkRight/BossWalkRight.BossWalkRight"))

(event `WalkRight`
  (`PaperFlipbookComponent.SetFlipbook` (`self.PaperFlipbook`) "/Game/Sprites/NPC/Boss/WalkRight/BossWalkRight.BossWalkRight"))

(event `Yell`
  (`PaperFlipbookComponent.SetFlipbook` (`self.PaperFlipbook`) "/Game/Sprites/NPC/Boss/Yell/BossYell.BossYell")
  (`GameplayStatics.PlaySoundAtLocation` "/Game/Sounds/Boss/AngruBoss_Cue.AngruBoss_Cue" (`SceneComponent.K2_GetComponentLocation` (`self.PaperFlipbook`)) (struct) 1.0 1.0 0.0 null null null null)
  (bind _asbp_player (cast `/Game/Blueprints/Player/BP_Player` (`GameplayStatics.GetPlayerCharacter` 0)))
  (set `/Game/Blueprints/Player/BP_Player.WasShoved` true _asbp_player))

(event `Idle`
  (`PaperFlipbookComponent.SetFlipbook` (`self.PaperFlipbook`) "/Game/Sprites/NPC/Boss/Idle/BossIdle.BossIdle"))

(event `Insult`)

(event `StopYell`
  (bind _asbp_player (cast `/Game/Blueprints/Player/BP_Player` (`GameplayStatics.GetPlayerCharacter` 0)))
  (set `/Game/Blueprints/Player/BP_Player.WasShoved` false _asbp_player))

(event `MakeFlamesAppear`
  (bind _returnvalue (`GameplayStatics.GetActorOfClass` "/Game/Blueprints/Player/BP_Player.BP_Player_C"))
  (`/Game/Blueprints/Player/BP_Player.MakeFlamesAppear` _returnvalue))

(fn `UserConstructionScript`)