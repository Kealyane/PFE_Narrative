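; Flame trigger for a small door that reacts to the player's flame value when the player overlaps it.
; A mid-range value briefly lights the flame and updates the affiliated door's activated-flame count, undoing both after a delay.
; A high value instead temporarily hides the scene root, without children, and disables box collision.
; A DoOnce gate blocks retriggering until either timed branch resets it; low values never reset it.
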(event `self.ReceiveActorBeginOverlap`
  (params (OtherActor :type "Actor Object Reference"))
  (bind _affiliateddoor (`self.AffiliatedDoor`))
  (bind _affiliateddoor_2 (`self.AffiliatedDoor`))
  (bind _asbp_player (cast `/Game/Blueprints/Player/BP_Player` OtherActor))
  (`/Engine/EditorBlueprintResources/StandardMacros.DoOnce` false :!label _label
    (:`Completed`
      (if (>= (`FlameComponent.GetFlameValue` (`/Game/Blueprints/Player/BP_Player.Flame` _asbp_player)) 70.0)
        (`SceneComponent.SetVisibility` (`self.DefaultSceneRoot`) false false)
        (`PrimitiveComponent.SetCollisionEnabled` (`self.Box`) "NoCollision")
        (`KismetSystemLibrary.Delay` 2.0)
        (`SceneComponent.SetVisibility` (`self.DefaultSceneRoot`) true false)
        (`PrimitiveComponent.SetCollisionEnabled` (`self.Box`) "QueryOnly")
        (`TypedElementListLibrary.Reset` (struct))
        (elif (not (<= (`FlameComponent.GetFlameValue` (`/Game/Blueprints/Player/BP_Player.Flame` _asbp_player)) 30.0))
          (`|ExecutionSequence`
            (:`then_0`
              (`SceneComponent.SetVisibility` (`self.Flame`) true false)
              (`/Engine/EditorBlueprintResources/StandardMacros.IncrementInt` (`/Game/Blueprints/Level/Doors/SmallDoorV1/BP_SmallFlameDoor.ActivatedFlames` _affiliateddoor_2)
                (:`  `
                  (`/Game/Blueprints/Level/Doors/SmallDoorV1/BP_SmallFlameDoor.CheckFlames` _affiliateddoor_2))))
            (:`then_1`
              (`KismetSystemLibrary.Delay` 2.0)
              (`SceneComponent.SetVisibility` (`self.Flame`) false false)
              (`/Engine/EditorBlueprintResources/StandardMacros.DecrementInt` (`/Game/Blueprints/Level/Doors/SmallDoorV1/BP_SmallFlameDoor.ActivatedFlames` _affiliateddoor)
                (:`  `
                  (`/Game/Blueprints/Level/Doors/SmallDoorV1/BP_SmallFlameDoor.CheckFlames` _affiliateddoor)
                  (`TypedElementListLibrary.Reset` (struct)))))))))))

(event `Reset`
  (goto _label :!via `Reset`))

(fn `UserConstructionScript`)