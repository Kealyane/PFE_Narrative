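; BP_SmallFlameDoor is a small 2D sprite door whose state depends on flame counts.
; BeginPlay zeroes ActivatedFlames; nothing here increments it or calls CheckFlames.
; CheckFlames shows the open sprite and sets the collider to overlap all channels while NumberOfFlames exceeds ActivatedFlames.
; Otherwise it shows the closed sprite and blocks all channels, so reaching the flame count closes the door.
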(event `self.ReceiveBeginPlay`
  (set `self.ActivatedFlames` 0))

(event `CheckFlames`
  (if (> (`self.NumberOfFlames`) (`self.ActivatedFlames`))
    (`PaperSpriteComponent.SetSprite` (`self.Door`) "/Game/Placeholder/PorteOuverte_Sprite.PorteOuverte_Sprite")
    (`PrimitiveComponent.SetCollisionResponseToAllChannels` (`self.Collider`) "ECR_Overlap")
    (else
      (`PaperSpriteComponent.SetSprite` (`self.Door`) "/Game/Placeholder/PorteFermee_Sprite.PorteFermee_Sprite")
      (`PrimitiveComponent.SetCollisionResponseToAllChannels` (`self.Collider`) "ECR_Block"))))

(fn `UserConstructionScript`)