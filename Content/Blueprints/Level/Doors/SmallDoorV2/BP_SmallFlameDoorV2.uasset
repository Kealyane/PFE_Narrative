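; BP_SmallFlameDoorV2 is a small sprite door that opens once enough flames are activated.
; On BeginPlay it creates a BP_DoorCounter widget on its widget component to show activated versus required flames.
; CheckFlames refreshes the counter, then either shows the closed sprite with blocking collision and visible counter, or shows the open sprite with overlap collision, plays a sound and hides the counter.
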(event `self.ReceiveBeginPlay`
  (set `self.ActivatedFlames` 0)
  (bind _returnvalue (`|CreateWidget` "/Game/Blueprints/Level/Doors/BP_DoorCounter.BP_DoorCounter_C"))
  (set `self.DoorCounter` _returnvalue)
  (`WidgetComponent.SetWidget` (`self.Widget`) _returnvalue)
  (set `/Game/Blueprints/Level/Doors/BP_DoorCounter.TotalFlames` (`KismetMathLibrary.Conv_IntToDouble` (`self.NumberOfFlames`)) _returnvalue)
  (set `/Game/Blueprints/Level/Doors/BP_DoorCounter.CurrentFlames` (`KismetMathLibrary.Conv_IntToDouble` (`self.ActivatedFlames`)) _returnvalue)
  (set `/Game/Blueprints/Level/Doors/BP_DoorCounter.IsSmallDoor` true _returnvalue)
  (`/Game/Blueprints/Level/Doors/BP_DoorCounter.CheckSliderColor` _returnvalue))

(event `CheckFlamesForWidget`
  (bind _doorcounter (`self.DoorCounter`))
  (set `/Game/Blueprints/Level/Doors/BP_DoorCounter.TotalFlames` (`KismetMathLibrary.Conv_IntToDouble` (`self.NumberOfFlames`)) _doorcounter)
  (set `/Game/Blueprints/Level/Doors/BP_DoorCounter.CurrentFlames` (`KismetMathLibrary.Conv_IntToDouble` (`self.ActivatedFlames`)) _doorcounter))

(event `CheckFlames`
  (`self.CheckFlamesForWidget`)
  (`/Game/Blueprints/Level/Doors/BP_DoorCounter.SetSlider` (`self.DoorCounter`))
  (if (> (`self.NumberOfFlames`) (`self.ActivatedFlames`))
    (`PaperSpriteComponent.SetSprite` (`self.Door`) "/Game/Sprites/Door/Porte_04_BW_Sprite_0.Porte_04_BW_Sprite_0")
    (`PrimitiveComponent.SetCollisionResponseToAllChannels` (`self.Collider`) "ECR_Block")
    (`SceneComponent.SetVisibility` (`self.Widget`) true false)
    (else
      (`PaperSpriteComponent.SetSprite` (`self.Door`) "/Game/Sprites/Door/Porte_04Open_Sprite_0.Porte_04Open_Sprite_0")
      (`PrimitiveComponent.SetCollisionResponseToAllChannels` (`self.Collider`) "ECR_Overlap")
      (`GameplayStatics.PlaySoundAtLocation` "/Game/Sounds/DoorSound_Cue.DoorSound_Cue" (`SceneComponent.K2_GetComponentLocation` (`self.DefaultSceneRoot`)) (struct) 1.0 1.0 0.0 null null null null)
      (`SceneComponent.SetVisibility` (`self.Widget`) false false))))

(fn `UserConstructionScript`)