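; Flame trigger actor for a small door, reacting to the player's flame value on overlap.
; A low value extinguishes the flame once and increments the linked door's activated count; a middle value relights it, decrements the count and resets the DoOnce.
; Either change makes the door recheck its flames.
; A high value instead hides the root component without propagation and disables box collision for a short delay.
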(event `self.ReceiveActorBeginOverlap`
  (params (OtherActor :type "Actor Object Reference"))
  (bind _affiliateddoor (`self.AffiliatedDoor`))
  (bind _affiliateddoor_2 (`self.AffiliatedDoor`))
  (bind _asbp_player (cast `/Game/Blueprints/Player/BP_Player` OtherActor))
  (set `self.PlayerRef` _asbp_player)
  (if (>= (`FlameComponent.GetFlameValue` (`/Game/Blueprints/Player/BP_Player.Flame` _asbp_player)) 70.0)
    (`SceneComponent.SetVisibility` (`self.DefaultSceneRoot`) false false)
    (`PrimitiveComponent.SetCollisionEnabled` (`self.Box`) "NoCollision")
    (`KismetSystemLibrary.Delay` 2.0)
    (`SceneComponent.SetVisibility` (`self.DefaultSceneRoot`) true false)
    (`PrimitiveComponent.SetCollisionEnabled` (`self.Box`) "QueryOnly")
    (elif (<= (`FlameComponent.GetFlameValue` (`/Game/Blueprints/Player/BP_Player.Flame` _asbp_player)) 30.0)
      (`/Engine/EditorBlueprintResources/StandardMacros.DoOnce` false :!label _label
        (:`Completed`
          (`SceneComponent.SetVisibility` (`self.Flame`) false false)
          (`/Engine/EditorBlueprintResources/StandardMacros.IncrementInt` (`/Game/Blueprints/Level/Doors/SmallDoorV2/BP_SmallFlameDoorV2.ActivatedFlames` _affiliateddoor)
            (:`  `
              (set `self.Out` true)
              (`/Game/Blueprints/Level/Doors/SmallDoorV2/BP_SmallFlameDoorV2.CheckFlames` _affiliateddoor)))))
      (elif (`self.Out`)
        (`SceneComponent.SetVisibility` (`self.Flame`) true false)
        (set `self.Out` false)
        (`/Engine/EditorBlueprintResources/StandardMacros.DecrementInt` (`/Game/Blueprints/Level/Doors/SmallDoorV2/BP_SmallFlameDoorV2.ActivatedFlames` _affiliateddoor_2)
          (:`  `
            (`/Game/Blueprints/Level/Doors/SmallDoorV2/BP_SmallFlameDoorV2.CheckFlames` _affiliateddoor_2)
            (`TypedElementListLibrary.Reset` (struct))))))))

(event `Reset`
  (goto _label :!via `Reset`))

(fn `UserConstructionScript`)