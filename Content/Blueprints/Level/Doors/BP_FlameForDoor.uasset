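; A brazier actor that the player lights or extinguishes on overlap, updating the active flame count on its affiliated door.
; Player flame values at or below the low threshold put out a lit brazier; mid-range values light it through a resettable DoOnce, and both trigger the door's flame check.
; High values spawn an explosion, hide pedestal and flame, then restore the pedestal and collision after a delay without updating the door.
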(event `self.ReceiveActorBeginOverlap`
  (params (OtherActor :type "Actor Object Reference"))
  (bind _affiliateddoor (`self.AffiliatedDoor`))
  (bind _affiliateddoor_2 (`self.AffiliatedDoor`))
  (bind _asbp_player (cast `/Game/Blueprints/Player/BP_Player` OtherActor))
  (if (<= (`FlameComponent.GetFlameValue` (`/Game/Blueprints/Player/BP_Player.Flame` _asbp_player)) 30.0)
    (if (`self.On`)
      (`SceneComponent.SetVisibility` (`self.Flame`) false false)
      (set `self.On` false)
      (`/Engine/EditorBlueprintResources/StandardMacros.DecrementInt` (`/Game/Blueprints/Level/Doors/BP_FlameDoor.ActivatedFlames` _affiliateddoor)
        (:`  `
          (`GameplayStatics.PlaySoundAtLocation` "/Game/Sounds/BraseroOut.BraseroOut" (`SceneComponent.K2_GetComponentLocation` (`self.DefaultSceneRoot`)) (struct) 1.0 1.0 0.0 null null null null)
          (`/Game/Blueprints/Level/Doors/BP_FlameDoor.CheckFlames` _affiliateddoor)
          (`self.Reset`))))
    (elif (>= (`FlameComponent.GetFlameValue` (`/Game/Blueprints/Player/BP_Player.Flame` _asbp_player)) 70.0)
      (`self.Burnt`)
      (else
        (`/Engine/EditorBlueprintResources/StandardMacros.DoOnce` false :!label _label
          (:`Completed`
            (`SceneComponent.SetVisibility` (`self.Flame`) true false)
            (set `self.On` true)
            (`GameplayStatics.PlaySoundAtLocation` "/Game/Sounds/BraseroLit.BraseroLit" (`SceneComponent.K2_GetComponentLocation` (`self.DefaultSceneRoot`)) (struct) 1.0 1.0 0.0 null null null null)
            (`/Engine/EditorBlueprintResources/StandardMacros.IncrementInt` (`/Game/Blueprints/Level/Doors/BP_FlameDoor.ActivatedFlames` _affiliateddoor_2)
              (:`  `
                (`/Game/Blueprints/Level/Doors/BP_FlameDoor.CheckFlames` _affiliateddoor_2)))))))))

(event `LightBrasero`
  (goto _label))

(event `Reset`
  (goto _label :!via `Reset`))

(event `Burnt`
  (bind (_returnvalue_x _returnvalue_y _returnvalue_z) (`KismetMathLibrary.BreakVector` (`SceneComponent.K2_GetComponentLocation` (`self.DefaultSceneRoot`))))
  (bind _returnvalue (`|SpawnActorFromClass` "/Game/Blueprints/Misc/PlayerExplosion.PlayerExplosion_C" (`KismetMathLibrary.MakeTransform` (`KismetMathLibrary.MakeVector` _returnvalue_x 1009.0 _returnvalue_z) (struct) (3.0 3.0 3.0)) "Undefined" "MultiplyWithRoot" null null))
  (`/Game/Blueprints/Misc/PlayerExplosion.Called` _returnvalue)
  (`GameplayStatics.PlaySoundAtLocation` "/Game/Sounds/BraseroExploded.BraseroExploded" (`SceneComponent.K2_GetComponentLocation` (`self.DefaultSceneRoot`)) (struct) 1.0 1.0 0.0 null null null null)
  (`KismetSystemLibrary.Delay` 0.2)
  (`SceneComponent.SetVisibility` (`self.Pedestal`) false false)
  (`SceneComponent.SetVisibility` (`self.Flame`) false false)
  (`PrimitiveComponent.SetCollisionEnabled` (`self.Box`) "NoCollision")
  (`KismetSystemLibrary.Delay` 2.0)
  (`SceneComponent.SetVisibility` (`self.Pedestal`) true false)
  (`PrimitiveComponent.SetCollisionEnabled` (`self.Box`) "QueryOnly"))

(fn `UserConstructionScript`)