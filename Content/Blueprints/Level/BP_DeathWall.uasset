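; Moving death wall that advances toward a Destination component and triggers the death event when it touches the player.
; BeginPlay adds the Destination's world location as an InterpToMovement control point, and the player overlapping Trigger activates that movement.
; The player overlapping Collision calls LaunchDeathEvent on BP_PFEGameMode, then stops the wall after a short delay.
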(event `self.ReceiveBeginPlay`
  (`InterpToMovementComponent.AddControlPointPosition` (`self.InterpToMovement`) (`SceneComponent.K2_GetComponentLocation` (`self.Destination`)) false))

(event `self.Collision.OnComponentBeginOverlap`
  (params (OverlappedComponent :type "PrimitiveComponent Object Reference") (OtherActor :type "Actor Object Reference") (OtherComp :type "PrimitiveComponent Object Reference") (OtherBodyIndex :type Integer) (bFromSweep :type Boolean) (SweepResult :type "HitResult Structure (by ref)"))
  (cast `/Game/Blueprints/Player/BP_Player` OtherActor)
  (bind _asbp_pfegame_mode (cast `/Game/Blueprints/Core/BP_PFEGameMode` (`GameplayStatics.GetGameMode`)))
  (`PFEGameMode.LaunchDeathEvent` _asbp_pfegame_mode)
  (`KismetSystemLibrary.Delay` 0.2)
  (`InterpToMovementComponent.StopSimulating` (`self.InterpToMovement`) SweepResult))

(event `self.Trigger.OnComponentBeginOverlap`
  (params (OverlappedComponent :type "PrimitiveComponent Object Reference") (OtherActor :type "Actor Object Reference") (OtherComp :type "PrimitiveComponent Object Reference") (OtherBodyIndex :type Integer) (bFromSweep :type Boolean) (SweepResult :type "HitResult Structure (by ref)"))
  (cast `/Game/Blueprints/Player/BP_Player` OtherActor)
  (`ActorComponent.Activate` (`self.InterpToMovement`) false))

(fn `UserConstructionScript`)